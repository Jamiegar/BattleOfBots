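; Shared viewport camera that keeps the group of player characters framed as they move.
; Init takes the character list from the game mode's message.
; Each tick it lerps its sphere toward the characters' average location by a fixed alpha, independent of delta time.
; It then sets spring arm length to the largest pairwise character distance, clamped between minimum and maximum camera distances, zooming out as players spread.
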(event `/Game/Jamie/Interfaces/GameMode/BPI_Initalize.Init`
  (bind _currentgamemode (message `/Game/Jamie/Interfaces/GameMode/BPI_GameMode.GetGameMode` (`GameplayStatics.GetGameMode`)))
  (set `self.characters` (`/Game/Jamie/Blueprint/GameMode/GM_Base_BrawlOfBots.character` _currentgamemode)))

(event `self.ReceiveTick`
  (params (DeltaSeconds :type "Float (single-precision)"))
  (`self.CalcCamreaMovement`)
  (`self.CalcSprinArmLength`))

(fn `CalcCamreaMovement`
  (bind _returnvalue (`GameplayStatics.GetActorArrayAverageLocation` (`self.characters`)))
  (`SceneComponent.K2_SetWorldLocation` (`self.Sphere`) (`KismetMathLibrary.VLerp` (`SceneComponent.K2_GetComponentLocation` (`self.Sphere`)) _returnvalue (`self.cameraMoveSpeed`)) false false))

(fn `CalcSprinArmLength`
  (locals (currentPlayer :type "Actor Object Reference") (distance :type "Array of Float (double-precision)"))
  (for _array_element (`self.characters`)
    (set `local.currentPlayer` _array_element)
    (for _index (range (`KismetArrayLibrary.Array_Length` (`self.characters`)))
      (`KismetArrayLibrary.Array_Add` (`local.distance`) (`self.GetDistanceTo` (`local.currentPlayer`) (`|GetArrayItem` (`self.characters`) _index)))))
  (set `SpringArmComponent.TargetArmLength` (`KismetMathLibrary.FClamp` (`.MaxValue` (`KismetMathLibrary.MaxOfFloatArray` (`local.distance`))) (`self.minCameraDistance`) (`self.maxCameraDistance`)) (`self.SpringArm`))
  (`KismetArrayLibrary.Array_Clear` (`local.distance`)))

(fn `UserConstructionScript`)