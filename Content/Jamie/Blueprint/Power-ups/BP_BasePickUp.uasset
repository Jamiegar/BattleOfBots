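; BP_BasePickUp is a base pickup that gives a named power-up to characters touching its sphere.
; On overlap with a BPI_Character implementer, it fetches the power-up by name from the game mode's power-up manager, notifies it of the pickup and passes it to the character to equip.
; The name is set through InitPickUp, and a usage flag is exposed through SetUsage and GetUsage but not changed on overlap.
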(event `/Game/Jamie/Interfaces/Power-up/BPI_PickUp.InitPickUp`
  (params (PowerUpName :type Name))
  (set `self.powerUpName` PowerUpName))

(event `self.Sphere.OnComponentBeginOverlap`
  (params (OverlappedComponent :type "PrimitiveComponent Object Reference") (OtherActor :type "Actor Object Reference") (OtherComp :type "PrimitiveComponent Object Reference") (OtherBodyIndex :type Integer) (bFromSweep :type Boolean) (SweepResult :type "HitResult Structure (by ref)"))
  (if (`KismetSystemLibrary.DoesImplementInterface` OtherActor "/Game/Jamie/Interfaces/Character/BPI_Character.BPI_Character_C")
    (bind _powerupmanager (message `/Game/Jamie/Interfaces/GameMode/BPI_GameMode.GetPowerUpManger` (`GameplayStatics.GetGameMode`)))
    (bind _powerup (`/Game/Jamie/Blueprint/Managers/BP_PowerupManager.GetPowerUp` _powerupmanager (`self.powerUpName`)))
    (message `/Game/Jamie/Interfaces/Power-up/BPI_Powerup.OnPickUp` _powerup)
    (message `/Game/Jamie/Interfaces/Character/BPI_Character.EquipItem` OtherActor _powerup)))

(event `/Game/Jamie/Interfaces/Power-up/BPI_Usable.SetUsage`
  (params (IsUsed :type Boolean))
  (set `self.isUsed` IsUsed))

(fn `GetUsage`
  (returns (isUsed :type Boolean))
  (return (`self.isUsed`)))

(fn `UserConstructionScript`)