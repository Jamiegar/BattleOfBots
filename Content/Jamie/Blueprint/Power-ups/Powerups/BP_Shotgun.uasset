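; BP_Shotgun is a power-up Blueprint that fires a spread of pellets when activated.
; Each pellet is a line trace along a random direction in an elliptical cone around the mesh's forward vector, sized by horizontal and vertical spread values.
; Every trace sends a ragdoll message to its hit actor, then the parent activation logic runs.
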(event `/Game/Jamie/Interfaces/Power-up/BPI_Powerup.ActivatePowerUp`
  (for _ (range (+ (`self.numOfPellets`) 1))
    (bind _linetracehit (`self.FireLineTrace` (`KismetMathLibrary.RandomUnitVectorInEllipticalConeInDegrees` (`SceneComponent.GetForwardVector` (`self.StaticMesh`)) (* (`self.spreadH`) 2.0) (* (`self.spreadV`) 2.0))))
    (message `/Game/Callum/BPI/BPI_playerChar.Activate Ragdoll` (`.HitActor` (`GameplayStatics.BreakHitResult` _linetracehit))))
  (`parent.ActivatePowerUp`))

(fn `UserConstructionScript`)