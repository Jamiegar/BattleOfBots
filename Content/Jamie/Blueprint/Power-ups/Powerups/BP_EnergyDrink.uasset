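; BP_EnergyDrink is a power-up that temporarily changes the interacting character's walk speed and jump height.
; On activation it plays a used VFX, applies the energy drink values through the character's message reference and starts a one-shot timer.
; OnEnergyDrinkEnd restores default movement and jump, deferring the parent ActivatePowerUp call until the effect ends.
; A character-state message call is left unconnected.
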(event `/Game/Jamie/Interfaces/Power-up/BPI_Powerup.ActivatePowerUp`
  (`self.PlayUsedVFX` (`self.K2_GetActorLocation`) (struct) (1.0 1.0 1.0))
  (bind _character (message `/Game/Jamie/Interfaces/Character/BPI_Character.GetCharacter` (`self.interactedCharacter`)))
  (`/Engine/EditorBlueprintResources/StandardMacros.IsValid` _character
    (:`Is Valid`
      ;[1 1 1] Change movement speed and jump height for character
      (`/Game/Callum/Characters/BP_BotCharacter.SetMovementSpeed` _character (`self.energyDrinkWalkSpeed`))
      (`/Game/Callum/Characters/BP_BotCharacter.SetJumpHeight` _character (`self.energyDrinkJumpHeight`))
      ;[1 1 1] Set a timer for duration of energy drink
      (`KismetSystemLibrary.K2_SetTimerDelegate` (`|CreateDelegate` :!event `OnEnergyDrinkEnd`) (`self.energyTimer`)))))

(event `OnEnergyDrinkEnd`
  ;[1 1 1] Return movement speed and jump height back to defaults when duration is done
  (bind _character (message `/Game/Jamie/Interfaces/Character/BPI_Character.GetCharacter` (`self.interactedCharacter`)))
  (`/Engine/EditorBlueprintResources/StandardMacros.IsValid` _character
    (:`Is Valid`
      (`/Game/Callum/Characters/BP_BotCharacter.SetMovementToDefault` _character)
      (`/Game/Callum/Characters/BP_BotCharacter.SetJumpToDefault` _character)
      (`parent.ActivatePowerUp`))))

(fn `UserConstructionScript`
  (`parent.UserConstructionScript`))