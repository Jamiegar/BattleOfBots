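; BP_Sniper is a power-up that fires a hitscan shot at a character in the front arc.
; On activation it plays a water-gun sound, takes the first character found, and line-traces from the fire point toward it.
; It sends the ragdoll message to whatever actor the trace hits.
; The parent activation runs only when a target is found, though the sound always plays.
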(event `/Game/Jamie/Interfaces/Power-up/BPI_Powerup.ActivatePowerUp`
  (`GameplayStatics.PlaySound2D` "/Game/Callum/Music/Sounds/Water_Gun_Shot.Water_Gun_Shot" 1.0 1.0 0.0 null null)
  (bind _characters_within_arc (`self.FindCharactersInFrontArc`)) ; Get charcters that are infrount of the charcter
  (bind _output (`|GetArrayItem` _characters_within_arc))
  (`/Engine/EditorBlueprintResources/StandardMacros.IsValid` _output
    (:`Is Valid`
      (bind _linetracehit (`self.FireLineTrace` (`KismetMathLibrary.GetDirectionUnitVector` (`self.GetFirePoint`) (`SceneComponent.K2_GetComponentLocation` (`Actor.RootComponent` _output)))))
      (message `/Game/Callum/BPI/BPI_Ragdoll.Activate Ragdoll` (`.HitActor` (`GameplayStatics.BreakHitResult` _linetracehit)))
      (`parent.ActivatePowerUp`))))

(fn `UserConstructionScript`)