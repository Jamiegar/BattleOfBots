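; BP_MirrorTime is a power-up that inverts the controls of every other character for a limited time.
; On activation it plays the used VFX at its location, then sends each other character a state message for inverted controls and starts a one-shot timer of TimeDuration.
; OnMirrorTimeEnd returns the other characters to their default state, and only then calls the parent ActivatePowerUp.
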(event `/Game/Jamie/Interfaces/Power-up/BPI_Powerup.ActivatePowerUp`
  ;[1 1 1] Set all other characters to have inverted controlls
  (`self.PlayUsedVFX` (`self.K2_GetActorLocation`) (struct) (1.0 1.0 1.0))
  (bind _characters (`self.GetAllOtherCharacters`))
  (for _array_element _characters
    (message `/Game/Jamie/Interfaces/Character/BPI_Character.SetCharacterState` _array_element "NewEnumerator2"))
  ;[1 1 1] Set timer for length of power up
  (`KismetSystemLibrary.K2_SetTimerDelegate` (`|CreateDelegate` :!event `OnMirrorTimeEnd`) (`self.TimeDuration`)))

(event `OnMirrorTimeEnd`
  ;[1 1 1] Set other characters back to default state after power up
  (bind _characters (`self.GetAllOtherCharacters`))
  (for _array_element _characters
    (message `/Game/Jamie/Interfaces/Character/BPI_Character.SetCharacterState` _array_element "NewEnumerator0"))
  (`parent.ActivatePowerUp`))

(fn `UserConstructionScript`
  (`parent.UserConstructionScript`))