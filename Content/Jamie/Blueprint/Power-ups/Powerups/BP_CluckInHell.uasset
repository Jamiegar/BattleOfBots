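; BP_CluckInHell is a thrown explosive power-up that ragdolls and launches nearby bots.
; While held, Tick debug-draws a predicted arc toward either the closest character in the front arc or a point ahead, depending on TargetClosestPlayer.
; Activation physically launches the mesh along that arc.
; On hit it explodes in a radius, resets and calls parent activation; spawned path markers and pooling are unwired.
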(event `/Game/Jamie/Interfaces/Power-up/BPI_Powerup.InitPowerUp`
  (params (PowerUpName :type Name))
  (`parent.InitPowerUp` PowerUpName))

(event `/Game/Jamie/Interfaces/Power-up/BPI_Powerup.OnPickUp`
  (params (`Interacted Character` :type "Actor Object Reference"))
  ;[1 1 1] Debug
  (`parent.OnPickUp` `Interacted Character`)
  (`KismetSystemLibrary.Delay` 0.2)
  (`self.K2_SetActorRelativeLocation` (100.0 0.0 0.0)))

(event `self.ReceiveTick`
  (params (DeltaSeconds :type "Float (single-precision)"))
  (bind _returnvalue (`SceneComponent.K2_GetComponentLocation` (`self.DefaultSceneRoot`)))
  (`parent.ReceiveTick` DeltaSeconds)
  (`/Engine/EditorBlueprintResources/StandardMacros.IsValid` (`self.interactedCharacter`)
    (:`Is Valid`
      (`self.ClearProdictedPath`)
      (if (`self.targetClosestPlayer`)
        (bind _characters_within_arc (`self.FindCharactersInFrontArc`)) ; Gets the characters in front of the interacted\ncharacter
        (if (`KismetArrayLibrary.Array_IsValidIndex` _characters_within_arc)
          (bind _closest (`self.GetClosestTargetFromArray` _characters_within_arc)) ; Get closest target from characters found\nin front of interacted character
          (bind _output_get (set `self.target` _closest)) ; Set target
          (`/Engine/EditorBlueprintResources/StandardMacros.IsValid` _output_get ; if it is valid then suggest a projectile path
            (:`Is Valid`
              ;[1 1 1] Suggest path and draw debug
              (bind _outlaunchvelocity (`GameplayStatics.SuggestProjectileVelocity_CustomArc` (`SceneComponent.K2_GetComponentLocation` (`self.DefaultSceneRoot`)) (`SceneComponent.K2_GetComponentLocation` (`Actor.RootComponent` _output_get))))
              (`GameplayStatics.Blueprint_PredictProjectilePath_ByTraceChannel` (`SceneComponent.K2_GetComponentLocation` (`self.DefaultSceneRoot`)) _outlaunchvelocity true 10.0 "ECC_WorldStatic" false (`|MakeArray` self (`self.interactedCharacter`) :!type "Actor Object Reference") "ForOneFrame")))
          (else
            (set `self.target` null)))
        (else
          (bind _output_get_2 (set `self.endPosition` (+ (* (`self.GetActorForwardVector`) (`self.range`)) _returnvalue))) ; Calculate end position based from\nactors foward vector
          ;[1 1 1] Suggest path and draw debug
          (bind _outlaunchvelocity_2 (`GameplayStatics.SuggestProjectileVelocity_CustomArc` _returnvalue _output_get_2))
          (`GameplayStatics.Blueprint_PredictProjectilePath_ByTraceChannel` (`SceneComponent.K2_GetComponentLocation` (`self.DefaultSceneRoot`)) _outlaunchvelocity_2 true 10.0 "ECC_WorldStatic" false (`|MakeArray` self (`self.interactedCharacter`) :!type "Actor Object Reference") "ForOneFrame"))))))

(event `/Game/Jamie/Interfaces/Power-up/BPI_Powerup.ActivatePowerUp`
  (bind _target (`self.target`))
  (if (`self.targetClosestPlayer`)
    ;[1 1 1] Through at target
    (`/Engine/EditorBlueprintResources/StandardMacros.IsValid` _target
      (:`Is Valid`
        (`self.ThrowAtTarget` (`self.K2_GetActorLocation` _target))))
    (else
      ;[1 1 1] Through at end position
      (`self.ThrowAtTarget` (`self.endPosition`)))))

(event `self.StaticMesh.OnComponentHit`
  (params (HitComponent :type "PrimitiveComponent Object Reference") (OtherActor :type "Actor Object Reference") (OtherComp :type "PrimitiveComponent Object Reference") (NormalImpulse :type "Vector Structure") (Hit :type "HitResult Structure (by ref)"))
  (bind _staticmesh (`self.StaticMesh`))
  (`KismetSystemLibrary.PrintString` (`KismetSystemLibrary.GetDisplayName` OtherActor))
  (`self.Explode` (`.Location` (`GameplayStatics.BreakHitResult` Hit))) ; On hit explode
  ;[1 1 1] Reset and recycle power up
  (`PrimitiveComponent.SetSimulatePhysics` _staticmesh false)
  (`SceneComponent.ResetRelativeTransform` _staticmesh)
  (`parent.ActivatePowerUp`))

(event `Explode`
  (params (StartPosition :type "Vector Structure"))
  (bind (_outactors _returnvalue) (`KismetSystemLibrary.SphereOverlapActors` StartPosition (`self.explosionRadius`) (`|MakeArray` "ObjectTypeQuery3" :!type "EObjectTypeQuery Enum") "/Game/Callum/Characters/BP_BotCharacter.BP_BotCharacter_C")) ; Explosion radius
  (`KismetSystemLibrary.DrawDebugSphere` StartPosition (`self.explosionRadius`) 12 (struct :`R` 1.0 :`G` 0.004929 :`A` 1.0) 2.0) ; Debug
  (if _returnvalue
    ;[1 1 1] Activate ragdoll
    (for _array_element _outactors
      (if (`KismetSystemLibrary.DoesImplementInterface` _array_element "/Game/Callum/BPI/BPI_Ragdoll.BPI_Ragdoll_C")
        (message `/Game/Callum/BPI/BPI_Ragdoll.Activate Ragdoll` _array_element)
        ;[1 1 1] Adds impulse to player for explosion
        (bind _character (message `/Game/Jamie/Interfaces/Character/BPI_Character.GetCharacter` _array_element))
        (bind _mesh (`Character.Mesh` _character))
        (if (`SceneComponent.IsSimulatingPhysics` _mesh "None")
          (`PrimitiveComponent.AddImpulseAtLocation` _mesh (* (`KismetMathLibrary.GetDirectionUnitVector` (`self.K2_GetActorLocation`) (`SceneComponent.K2_GetComponentLocation` _mesh)) (`self.explosionForce`)) StartPosition "None") ; Add Impuse from direction of impact
        )))))

(fn `ClearProdictedPath`
  (bind _values (`BlueprintMapLibrary.Map_Values` (`self.path`)))
  (if (`KismetArrayLibrary.Array_IsValidIndex` _values)
    (for _array_element _values
      (`self.K2_DestroyActor` _array_element))
    (`BlueprintMapLibrary.Map_Clear` (`self.path`))))

(fn `ShowProdictedPath`
  (params (Path :type "Array of Vector Structure"))
  (for _array_element Path
    (bind _returnvalue (`|SpawnActorFromClass` "/Game/Jamie/Blueprint/BP_PathProdict.BP_PathProdict_C" (`KismetMathLibrary.MakeTransform` _array_element) "Undefined" "OverrideRootScale" null null))
    (`BlueprintMapLibrary.Map_Add` (`self.path`) _array_element _returnvalue)))

(fn `ThrowAtTarget`
  (params (Position :type "Vector Structure"))
  (bind (_outlaunchvelocity _returnvalue) (`GameplayStatics.SuggestProjectileVelocity_CustomArc` (`SceneComponent.K2_GetComponentLocation` (`self.DefaultSceneRoot`)) Position))
  (if _returnvalue
    (`PrimitiveComponent.SetSimulatePhysics` (`self.StaticMesh`) true)
    (`PrimitiveComponent.AddImpulse` (`self.StaticMesh`) _outlaunchvelocity "None" true)))

(fn `UserConstructionScript`)