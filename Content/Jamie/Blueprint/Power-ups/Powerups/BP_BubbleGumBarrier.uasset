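; BP_BubbleGumBarrier is a power-up that acts as a one-time block against a particular character state.
; On activation it binds to the interacted character's state-change event through its character message object, deferring the parent activation.
; When the blocked state arrives, it sets the character to another state, unbinds, then runs the parent ActivatePowerUp logic.
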(event `/Game/Jamie/Interfaces/Power-up/BPI_Powerup.ActivatePowerUp`
  (bind _character (message `/Game/Jamie/Interfaces/Character/BPI_Character.GetCharacter` (`self.interactedCharacter`)))
  (add `/Game/Callum/Characters/BP_BotCharacter.OnStateChanged` _character (`|CreateDelegate` :!event `Block`)))

(event `Block`
  (params (`New State` :type "/Game/Jamie/Blueprint/Characters/Enum_CharacterStates Enum" :default "NewEnumerator0") (`Last State` :type "/Game/Jamie/Blueprint/Characters/Enum_CharacterStates Enum" :default "NewEnumerator0"))
  (if (`|EnumEquality` `New State` "NewEnumerator3")
    (message `/Game/Jamie/Interfaces/Character/BPI_Character.SetCharacterState` (`self.interactedCharacter`) "NewEnumerator0")
    (bind _character (message `/Game/Jamie/Interfaces/Character/BPI_Character.GetCharacter` (`self.interactedCharacter`)))
    (remove `/Game/Callum/Characters/BP_BotCharacter.OnStateChanged` _character (`|CreateDelegate` :!event `Block`))
    (`parent.ActivatePowerUp`)))

(fn `UserConstructionScript`)