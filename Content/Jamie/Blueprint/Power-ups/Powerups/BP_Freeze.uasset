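; BP_Freeze is a power-up that temporarily makes a character in front slippery by changing its movement friction.
; On activation it takes the first result of FindCharactersInFrontArc, caches that character's ground friction and walking braking deceleration, then applies the freeze values and starts a one-shot timer.
; DeactivateFreeze restores the cached values and only then calls the parent ActivatePowerUp.
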(event `/Game/Jamie/Interfaces/Power-up/BPI_Powerup.ActivatePowerUp`
  (bind _characters_within_arc (`self.FindCharactersInFrontArc`))
  (bind _output_get (set `self.traget` (`|GetArrayItem` _characters_within_arc)))
  (bind _character (message `/Game/Jamie/Interfaces/Character/BPI_Character.GetCharacter` _output_get))
  (bind _charactermovement (`Character.CharacterMovement` _character))
  (set `self.DefaultGroundFiction` (`CharacterMovementComponent.GroundFriction` _charactermovement))
  (set `self.DefaultBreakingWalking` (`CharacterMovementComponent.BrakingDecelerationWalking` _charactermovement))
  (bind _charactermovement_2 (`Character.CharacterMovement` _character))
  (set `CharacterMovementComponent.GroundFriction` (`self.FreezedGroundFriction`) _charactermovement_2)
  (set `CharacterMovementComponent.BrakingDecelerationWalking` (`self.BreakingDeceleration`) _charactermovement_2)
  (`KismetSystemLibrary.K2_SetTimerDelegate` (`|CreateDelegate` :!event `DeactivateFreeze`) (`self.FreezeTimer`)))

(event `DeactivateFreeze`
  (bind _character (message `/Game/Jamie/Interfaces/Character/BPI_Character.GetCharacter` (`self.traget`)))
  (bind _charactermovement (`Character.CharacterMovement` _character))
  (set `CharacterMovementComponent.GroundFriction` (`self.DefaultGroundFiction`) _charactermovement)
  (set `CharacterMovementComponent.BrakingDecelerationWalking` (`self.DefaultBreakingWalking`) _charactermovement)
  (`parent.ActivatePowerUp`))

(fn `UserConstructionScript`)