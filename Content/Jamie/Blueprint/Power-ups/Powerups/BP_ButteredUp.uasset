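; Buttered Up power-up that temporarily makes the interacting character impossible to grab.
; On activation, a DoOnce gate clears the character's CanBeGrabed flag, plays the used VFX and starts a one-shot timer lasting ButteredTimer.
; OnButteredUpEnd restores grabbing, resets the gate and only then calls the parent activation.
; An invalid character skips straight to the reset and parent call.
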(event `/Game/Jamie/Interfaces/Power-up/BPI_Powerup.ActivatePowerUp`
  (`/Engine/EditorBlueprintResources/StandardMacros.DoOnce` false :!label _label
    (:`Completed`
      (bind _character (message `/Game/Jamie/Interfaces/Character/BPI_Character.GetCharacter` (`self.interactedCharacter`)))
      (`/Engine/EditorBlueprintResources/StandardMacros.IsValid` _character
        (:`Is Valid`
          (set `/Game/Callum/Characters/BP_BotCharacter.canBeGrabed` false _character)
          (`self.PlayUsedVFX` (`self.K2_GetActorLocation`) (struct) (1.0 1.0 1.0))
          (`KismetSystemLibrary.K2_SetTimerDelegate` (`|CreateDelegate` :!event `OnButteredUpEnd`) (`self.butteredTimer`)))
        (:`Is Not Valid`
          (`self.ResetPowerUp`)
          (`parent.ActivatePowerUp`))))))

(event `ResetPowerUp`
  (goto _label :!via `Reset`))

(event `OnButteredUpEnd`
  (bind _character (message `/Game/Jamie/Interfaces/Character/BPI_Character.GetCharacter` (`self.interactedCharacter`)))
  (set `/Game/Callum/Characters/BP_BotCharacter.canBeGrabed` true _character)
  (`self.ResetPowerUp`)
  (`self.ResetPowerUp`)
  (`parent.ActivatePowerUp`))

(fn `UserConstructionScript`)