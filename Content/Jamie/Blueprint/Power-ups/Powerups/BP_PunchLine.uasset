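; BP_PunchLine is a power-up that knocks the player closest to its user away.
; On activation it runs the parent logic, finds the closest player and gets that player's character.
; It launches that character along the unit direction from the interacting character toward it, scaled by KnockBack, adding to its current velocity rather than overriding it.
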(event `/Game/Jamie/Interfaces/Power-up/BPI_Powerup.ActivatePowerUp`
  (`parent.ActivatePowerUp`)
  (bind _closestplayer (`self.FindClosestPlayer`)) ; Get the closest player
  (bind _character (message `/Game/Jamie/Interfaces/Character/BPI_Character.GetCharacter` _closestplayer))
  (`Character.LaunchCharacter` _character (* (`KismetMathLibrary.GetDirectionUnitVector` (`self.K2_GetActorLocation` (`self.interactedCharacter`)) (`self.K2_GetActorLocation` _closestplayer)) (`self.knockBack`)) false false))

(fn `UserConstructionScript`
  (`parent.UserConstructionScript`))