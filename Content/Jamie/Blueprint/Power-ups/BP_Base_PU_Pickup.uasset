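; Base power-up pickup, configured by name from the D_PowerUpData table; children override its activation, which here only prints and clears the in-use flag.
; On overlap with a BPI_Character actor, it either activates immediately or is handed to the character, depending on the row's trigger setting.
; Both paths then recycle the pickup through the game mode's power-up manager and fire the picked-up call.
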(event `self.InitPowerUp`
  (params (PowerUpName :type Name))
  ;[1 1 1] Init
  (set `self.powerUpName` PowerUpName)
  (`self.SetupVariables`))

(event `self.ActivatePowerUp`
  ;[1 1 1] This is the function that will be overriden in the child classes so that the power ups ability will happen. THis base class only prints what power up is being activated
  (`KismetSystemLibrary.PrintString` (`KismetStringLibrary.Concat_StrStr` (`KismetStringLibrary.Conv_NameToString` (`self.powerUpName`)) ": Power-Up has activated") true true (struct :`R` 1.0 :`G` 0.03824 :`A` 1.0))
  (set `self.inUse` false))

(event `self.PickupCollision.OnComponentBeginOverlap`
  (params (OverlappedComponent :type "PrimitiveComponent Object Reference") (OtherActor :type "Actor Object Reference") (OtherComp :type "PrimitiveComponent Object Reference") (OtherBodyIndex :type Integer) (bFromSweep :type Boolean) (SweepResult :type "HitResult Structure (by ref)"))
  ;[1 1 1] Collision Pickup
  (if (`KismetSystemLibrary.DoesImplementInterface` OtherActor "/Game/Jamie/Interfaces/Character/BPI_Character.BPI_Character_C")
    (if (`self.Trigged on Overlap`)
      ;[1 1 1] Trigger Power up on overlap
      (`self.ActivatePowerUp`)
      (`self.OnPowerUpPickUp` OtherActor)
      (else
        ;[1 1 1] Pick up power up to character
        (message `/Game/Jamie/Interfaces/Character/BPI_Character.Pickup Powerup` OtherActor self)
        (`self.OnPowerUpPickUp` OtherActor)))))

(event `self.SetUsage`
  (params (IsUsed :type Boolean))
  (set `self.inUse` IsUsed))

(fn `GetUsage`
  (returns (IsUsed :type Boolean))
  (return (`self.inUse`)))

(fn `OnPowerUpPickUp`
  (params (HitCharacter :type "Actor Object Reference"))
  ;[1 1 1] Recycle To Manager
  (bind _powerupmanager (message `/Game/Jamie/Interfaces/GameMode/BPI_GameMode.GetPowerUpManger` (`GameplayStatics.GetGameMode`)))
  (`/Game/Jamie/Blueprint/Managers/BP_PowerupManager.RecyclePowerUp` _powerupmanager (`self.powerUpName`) self)
  (`self.PowerUpPickedUP`)
  (`KismetSystemLibrary.PrintString` (`KismetStringLibrary.Concat_StrStr` (`KismetStringLibrary.Conv_NameToString` (`self.powerUpName`)) ": Power up picked up")))

(fn `SetupVariables`
  (bind _returnvalue (`|GetDataTableRow` "/Game/Jamie/DataTables/D_PowerUpData.D_PowerUpData" (`self.powerUpName`))
    (:`then`
      (bind (_name _uses _type _knockback _vfx _mesh _sfxwhenused _triggedonoverlap) (break `/Game/Jamie/Structs/StructsForDataTables/Struct_PowerUpData` _returnvalue))
      (set `self.uses` _uses)
      (set `self.powerUpType` _type)
      (set `self.knockBack` _knockback)
      (`StaticMeshComponent.SetStaticMesh` (`self.StaticMesh`) _mesh)
      (set `self.soundOnUse` _sfxwhenused)
      (set `self.Trigged on Overlap` _triggedonoverlap))))

(fn `UserConstructionScript`)