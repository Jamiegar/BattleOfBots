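; BP_BasePickUp is the base pickup actor that grants a named power-up to a character on overlap.
; InitPickUp sets its mesh from the D_PickUpsData table, disguising random pickups with a rotated random mesh, and enables query collision.
; On overlap with a BPI_Character actor, it gets the power-up from the game mode's manager, notifies and equips it, then disables collision and returns itself to the manager for recycling.
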(event `/Game/Jamie/Interfaces/Power-up/BPI_Pickup.InitPickUp`
  (params (PowerUpName :type Name))
  ;[1 1 1] Init Pick up, sets up the pick up for the power up
  (set `self.powerUpName` PowerUpName)
  (`self.SetUpPickUp`)
  (`PrimitiveComponent.SetCollisionEnabled` (`self.Sphere`) "QueryOnly"))

(event `self.Sphere.OnComponentBeginOverlap`
  (params (OverlappedComponent :type "PrimitiveComponent Object Reference") (OtherActor :type "Actor Object Reference") (OtherComp :type "PrimitiveComponent Object Reference") (OtherBodyIndex :type Integer) (bFromSweep :type Boolean) (SweepResult :type "HitResult Structure (by ref)"))
  ;[1 1 1] When character overlaps
  (if (`KismetSystemLibrary.DoesImplementInterface` OtherActor "/Game/Jamie/Interfaces/Character/BPI_Character.BPI_Character_C")
    (bind _powerupmanager (message `/Game/Jamie/Interfaces/GameMode/BPI_GameMode.GetPowerUpManger` (`GameplayStatics.GetGameMode`)))
    (bind _powerup (`/Game/Jamie/Blueprint/Managers/BP_PowerupManager.GetPowerUp` _powerupmanager (`self.powerUpName`))) ; Gets the power up
    (message `/Game/Jamie/Interfaces/Power-up/BPI_Powerup.OnPickUp` _powerup OtherActor) ; Runs on the power up to check if it needs \nto activate on pick up
    (message `/Game/Jamie/Interfaces/Character/BPI_Character.EquipItem` OtherActor _powerup) ; Equips the power up to the character\nby attaching it to the character
    ;;[1 1 1] Disable colksion so that when recycled it does not interact with anything else
    (`PrimitiveComponent.SetCollisionEnabled` (`self.Sphere`) "NoCollision")
    ;;[1 1 1] Recycle this pickup
    (bind _powerupmanager_2 (message `/Game/Jamie/Interfaces/GameMode/BPI_GameMode.GetPowerUpManger` (`GameplayStatics.GetGameMode`)))
    (`/Game/Jamie/Blueprint/Managers/BP_PowerupManager.RecyclePickUp` _powerupmanager_2 self)
    (`self.OnPickUp`)))

(event `/Game/Jamie/Interfaces/Power-up/BPI_Usable.SetUsage`
  (params (IsUsed :type Boolean))
  (set `self.isUsed` IsUsed))

(fn `GetUsage`
  (returns (isUsed :type Boolean))
  (return (`self.isUsed`)))

(fn `SetUpPickUp`
  (bind _returnvalue (`|GetDataTableRow` "/Game/Jamie/DataTables/D_PickUpsData.D_PickUpsData" (`self.powerUpName`))
    (:`then`
      (bind (_powerupname _pickupmesh _israndom) (break `/Game/Jamie/Structs/StructsForDataTables/Struct_PickUpData` _returnvalue))
      (if _israndom
        ;[1 1 1] Select random power up mesh
        (bind _outrownames (`DataTableFunctionLibrary.GetDataTableRowNames` "/Game/Jamie/DataTables/D_PickUpsData.D_PickUpsData")) ; Get all names in data table
        (bind _returnvalue_2 (`|GetDataTableRow` "/Game/Jamie/DataTables/D_PickUpsData.D_PickUpsData" (`|GetArrayItem` _outrownames (`KismetMathLibrary.RandomIntegerInRange` 0 (- (`KismetArrayLibrary.Array_Length` _outrownames) 1)))) ; Selects mesh
          (:`then`
            (`StaticMeshComponent.SetStaticMesh` (`self.StaticMesh`) (`.PickUpMesh_5_74BFC90E45921F52EFEF8895DB0DF5D1` (break `/Game/Jamie/Structs/StructsForDataTables/Struct_PickUpData` _returnvalue_2))) ; Set mesh
            (`SceneComponent.K2_SetRelativeRotation` (`self.StaticMesh`) (struct :`Pitch` -180.0) false false) ; rotate upside down
          ))
        (else
          (`StaticMeshComponent.SetStaticMesh` (`self.StaticMesh`) _pickupmesh))))))

(fn `UserConstructionScript`)