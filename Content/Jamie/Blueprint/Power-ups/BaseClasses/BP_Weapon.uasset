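; BP_Weapon is a weapon power-up Blueprint, filed among the power-up base classes, that provides shared firing helpers.
; GetFirePoint reads the world location of the Fire_Point socket on the static mesh.
; FireLineTrace casts a debug-drawn Visibility trace from that point along a given direction out to Range and returns the hit.
; Activation runs the parent logic, then only prints the fire point location.
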(event `/Game/Jamie/Interfaces/Power-up/BPI_Powerup.ActivatePowerUp`
  (`parent.ActivatePowerUp`)
  (`KismetSystemLibrary.PrintString` (`KismetStringLibrary.Conv_VectorToString` (`self.GetFirePoint`)) true true (struct :`R` 1.0 :`G` 0.845962 :`A` 1.0) 3.0))

(fn `FireLineTrace`
  (params (Direction :type "Vector Structure"))
  (returns (LineTraceHit :type "HitResult Structure"))
  (bind _firepointlocation (`self.GetFirePoint`))
  (bind _outhit (`KismetSystemLibrary.LineTraceSingle` :`Start` _firepointlocation :`End` (+ _firepointlocation (* Direction (`self.range`))) :`TraceChannel` "TraceTypeQuery1" :`DrawDebugType` "ForDuration" :`TraceColor` (struct :`G` 0.128125 :`B` 1.0 :`A` 1.0)))
  (return _outhit))

(fn `GetFirePoint`
  (returns (FirePointLocation :type "Vector Structure"))
  (return (`SceneComponent.GetSocketLocation` (`self.StaticMesh`) "Fire_Point")))

(fn `UserConstructionScript`
  (`parent.UserConstructionScript`))