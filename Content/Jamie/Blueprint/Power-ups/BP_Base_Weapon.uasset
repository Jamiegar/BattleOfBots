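; BP_Base_Weapon is a weapon power-up Blueprint that extends a parent power-up, passing activation, setup and construction straight through to it.
; On pickup it runs the parent logic, gets the power-up manager from the game mode through a message call, and looks up the weapon matching its power-up name.
; The node meant to equip the weapon on the character is disconnected, so pickup equips nothing here.
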(event `/Game/Jamie/Interfaces/Power-up/BPI_Powerup.ActivatePowerUp`
  (`parent.ActivatePowerUp`))

(fn `OnPowerUpPickUp`
  (params (HitCharacter :type "Actor Object Reference"))
  (`parent.OnPowerUpPickUp` HitCharacter)
  (bind _powerupmanager (message `/Game/Jamie/Interfaces/GameMode/BPI_GameMode.GetPowerUpManger` (`GameplayStatics.GetGameMode`))) ; Get a ref to the power-up manager
  (`/Game/Jamie/Blueprint/Managers/BP_PowerupManager.GetWeapon` _powerupmanager (`self.powerUpName`)) ; Get the weapon that has the same \nname as this power up
)

(fn `SetupVariables`
  (`parent.SetupVariables`))

(fn `UserConstructionScript`
  (`parent.UserConstructionScript`))