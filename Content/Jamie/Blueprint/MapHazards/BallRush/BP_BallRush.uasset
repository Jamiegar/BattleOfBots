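; BP_BallRush is a map hazard that opens doors, releases balls for a set time, then clears them away.
; Activation opens the doors and binds to their finished event, while a separate event spawns BP_Balls at an offset from the actor and starts the hazard-length timer.
; Stopping the hazard destroys the spawned balls actor, unbinds from the door event and closes the doors.
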(event `/Game/Jamie/Interfaces/Map/BPI_MapHazards.StopMapHazard`
  ;[1 1 1] Hazard stops
  (`self.K2_DestroyActor` (`self.balls`))
  (remove `/Game/Callum/BP/BallRush/BP_LargeDoor.Doorfinished` (`self.Doors`) (`|CreateDelegate` :!event `Activate Balls`)) ; Unbind from doors event as this is no longer\nneeded
  (`/Game/Callum/BP/BallRush/BP_LargeDoor.CloseDoors` (`self.Doors`)))

(event `/Game/Jamie/Interfaces/Map/BPI_MapHazards.ActivateMapHazard`
  (bind _doors (`self.Doors`))
  ;[1 1 1] Activate Hazard
  (`/Game/Callum/BP/BallRush/BP_LargeDoor.OpenDoors` _doors)
  (add `/Game/Callum/BP/BallRush/BP_LargeDoor.Doorfinished` _doors (`|CreateDelegate` :!event `Activate Balls`)))

(event `Activate Balls`
  ;[1 1 1] Spawn Balls on spawn position and set length for hazard
  (bind _returnvalue (`|SpawnActorFromClass` "/Game/Callum/BP/BallRush/BP_Balls.BP_Balls_C" (`KismetMathLibrary.MakeTransform` (+ (`self.SpawnLocation`) (`self.K2_GetActorLocation`))) "Undefined" "OverrideRootScale" null null))
  (set `self.balls` _returnvalue)
  (`KismetSystemLibrary.K2_SetTimerDelegate` (`|CreateDelegate` :!event `StopMapHazard`) (`self.hazardLength`)))

(fn `UserConstructionScript`)