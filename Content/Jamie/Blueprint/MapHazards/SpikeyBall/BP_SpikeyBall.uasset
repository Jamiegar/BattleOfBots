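; Spikey ball map hazard that rolls under physics and ragdolls characters it overlaps, with a brief re-trigger cooldown.
; Activation enables physics and starts a looping timer for the default roll type.
; Rolls push the mesh with forces, either within a forward cone or toward a player randomly re-picked each call.
; Stopping disables physics, restores the start position, clears the timer and signals the hazard finished; debug mode draws a target line.
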(event `self.ReceiveTick`
  (params (DeltaSeconds :type "Float (single-precision)"))
  ;[1 1 1] Debug
  (`/Engine/EditorBlueprintResources/StandardMacros.Gate` true
    (:`Exit`
      (if (`self.debug`)
        (`KismetSystemLibrary.DrawDebugLine` (`SceneComponent.K2_GetComponentLocation` (`self.StaticMesh`)) (`self.K2_GetActorLocation` (`self.Target`)) (struct :`R` 1.0 :`B` 0.100525 :`A` 1.0) 0.0 1.5)))))

(event `/Game/Jamie/Interfaces/Map/BPI_MapFall.ResetActor`
  ;[1 1 1] Resets actor
  (`self.K2_SetActorLocation` (`self.intialStartPosition`)))

(event `/Game/Jamie/Interfaces/GameMode/BPI_Initalize.Init`
  ;[1 1 1] Begin Play
  (bind _currentgamemode (message `/Game/Jamie/Interfaces/GameMode/BPI_BotsGameMode.GetGameMode` (`GameplayStatics.GetGameMode`)))
  (set `self.Players` (`/Game/Jamie/Blueprint/GameMode/GM_Base_BrawlOfBots.character` _currentgamemode))
  (set `self.intialStartPosition` (`self.K2_GetActorLocation`)))

(event `/Game/Jamie/Interfaces/Map/BPI_MapHazards.ActivateMapHazard`
  (`PrimitiveComponent.SetSimulatePhysics` (`self.StaticMesh`) true)
  (`self.Change Roll Type` (`self.DefaultRollType`)))

(event `/Game/Jamie/Interfaces/Map/BPI_MapHazards.StopMapHazard`
  (`PrimitiveComponent.SetSimulatePhysics` (`self.StaticMesh`) false)
  (`self.K2_SetActorLocation` (`self.intialStartPosition`))
  (`KismetSystemLibrary.K2_ClearAndInvalidateTimerHandle` (`self.UpdateTimer`))
  (`self.OnHazardFinished`))

(event `self.Collision.OnComponentBeginOverlap`
  (params (OverlappedComponent :type "PrimitiveComponent Object Reference") (OtherActor :type "Actor Object Reference") (OtherComp :type "PrimitiveComponent Object Reference") (OtherBodyIndex :type Integer) (bFromSweep :type Boolean) (SweepResult :type "HitResult Structure (by ref)"))
  ;[1 1 1] Hit detection
  (`/Engine/EditorBlueprintResources/StandardMacros.DoOnce` false :!label _label
    (:`Completed`
      (if (`KismetSystemLibrary.DoesImplementInterface` OtherActor "/Game/Callum/BPI/BPI_Ragdoll.BPI_Ragdoll_C")
        (message `/Game/Callum/BPI/BPI_Ragdoll.Activate Ragdoll` OtherActor)
        (`KismetSystemLibrary.Delay` 0.2)
        (goto _label :!via `Reset`)))))

(fn `Change Roll Type`
  (params (`Roll Type` :type "/Game/Xan/Enum/Enum_RollTypes Enum" :default "NewEnumerator0"))
  (switch `/Game/Xan/Enum/Enum_RollTypes` `Roll Type`
    (:`NewEnumerator0`
      (bind _returnvalue (`KismetSystemLibrary.K2_SetTimerDelegate` (`|CreateDelegate` :!event `RollInRandomDirection`) 0.5 true))
      (set `self.UpdateTimer` _returnvalue))
    (:`NewEnumerator1`
      (bind _returnvalue_2 (`KismetSystemLibrary.K2_SetTimerDelegate` (`|CreateDelegate` :!event `RollToTargetPlayer`) 0.1 true))
      (set `self.UpdateTimer` _returnvalue_2))))

(fn `RollInRandomDirection`
  (bind (_returnvalue_x _returnvalue_y) (`KismetMathLibrary.BreakVector` (`KismetMathLibrary.RandomUnitVectorInConeInDegrees` (`self.GetActorForwardVector`) 45.0)))
  (`PrimitiveComponent.AddForce` (`self.StaticMesh`) (* (`KismetMathLibrary.MakeVector` _returnvalue_x _returnvalue_y) (`self.RollTorque`)) "None" false))

(fn `RollToTargetPlayer`
  (bind _playertargeted (`self.TargetRandomPlayer` (`self.Players`)))
  (set `self.Target` _playertargeted)
  (`PrimitiveComponent.AddForce` (`self.StaticMesh`) (* (`KismetMathLibrary.GetDirectionUnitVector` (`SceneComponent.K2_GetComponentLocation` (`self.StaticMesh`)) (`self.K2_GetActorLocation` (`self.Target`))) (`self.RollTorque`)) "None" false))

(fn `TargetRandomPlayer`
  (params (Players :type "Array of Actor Object Reference"))
  (returns (PlayerTargeted :type "Actor Object Reference"))
  (return (`|GetArrayItem` Players (`KismetMathLibrary.RandomIntegerInRange` 0 (- (`KismetArrayLibrary.Array_Length` Players) 1)))))

(fn `UserConstructionScript`)