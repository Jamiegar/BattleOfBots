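; BP_Manager is a manager actor that appears to serve as a base class, with an Init event and a duplicate-placement check.
; Init is a default stub that prints the actor's display name with a notice that it has no initialisation.
; The Construction Script searches for actors of the instance's own class and prints a red warning if more than one exists, without removing the duplicate.
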(event `/Game/Jamie/Interfaces/GameMode/BPI_Initalize.Init`
  (`KismetSystemLibrary.PrintString` (`KismetStringLibrary.Concat_StrStr` (`KismetSystemLibrary.GetDisplayName` self) " has no initalisation ") true true (struct :`R` 1.0 :`G` 0.844084 :`A` 1.0)))

(fn `UserConstructionScript`
  (bind _outactors (`GameplayStatics.GetAllActorsOfClass` (`GameplayStatics.GetObjectClass` self)))
  (if (> (`KismetArrayLibrary.Array_Length` _outactors) 1)
    (`KismetSystemLibrary.PrintString` "Manager Already in Scene" true true (struct :`R` 1.0 :`B` 0.009513 :`A` 1.0) 5.0)))