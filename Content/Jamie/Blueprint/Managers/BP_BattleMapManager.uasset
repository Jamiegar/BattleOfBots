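; BP_BattleMapManager is a battle map manager that, as written, only handles the reference to the player viewport camera.
; Its Init event finds the placed BP_PlayerViewportCamera when no valid reference is cached, and prints a warning if the level has none.
; A separate InitalizeCamera function sends InitMessage to the cached camera without a validity check, and nothing in this Blueprint calls it.
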(event `/Game/Jamie/Interfaces/GameMode/BPI_Initalize.Init`
  (`/Engine/EditorBlueprintResources/StandardMacros.IsValid` (`self.camrea`)
    (:`Is Not Valid`
      (`self.GetCameraInWorld`))))

(fn `GetCameraInWorld`
  (bind _returnvalue (`GameplayStatics.GetActorOfClass` "/Game/Jamie/Blueprint/Camera/BP_PlayerViewportCamera.BP_PlayerViewportCamera_C"))
  (`/Engine/EditorBlueprintResources/StandardMacros.IsValid` _returnvalue
    (:`Is Valid`
      (set `self.camrea` _returnvalue))
    (:`Is Not Valid`
      (`KismetSystemLibrary.PrintString` "place camera in world"))))

(fn `InitalizeCamera`
  (message `/Game/Jamie/Interfaces/GameMode/BPI_Initalize.Init` (`self.camrea`)))

(fn `UserConstructionScript`)