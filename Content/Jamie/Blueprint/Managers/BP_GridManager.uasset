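; Grid manager actor that builds a hex tile map in either a circular or square layout.
; Init triggers generation, which destroys old tiles, then measures node size from a temporary spawn's bounds.
; Circular layout builds two mirrored halves with per-row offsets and shrinking rows, while square layout staggers odd rows.
; Nodes are spaced at 75% row height, attached to the manager and stored in a map keyed by grid position.
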(event `self.ReceiveBeginPlay`)

(event `/Game/Jamie/Interfaces/GameMode/BPI_Initalize.Init`
  (`self.Genrate`))

(event `Genrate`
  (`self.Clear`)
  (`self.GetNodeDimentions`)
  (switch `/Game/Jamie/Enum/MapManger/Enum_MapStates` (`self.mapGenrationType`)
    (:`NewEnumerator0`
      (`self.GenrateCircularGrid`))
    (:`NewEnumerator1`
      (`self.GenrateSquareGrid`))))

(event `Clear`
  ;[1 1 1] Clears all the nodes and destroys all the nodes
  (bind _values (`BlueprintMapLibrary.Map_Values` (`self.tiles`)))
  (for _array_element _values
    (`self.K2_DestroyActor` _array_element))
  (`BlueprintMapLibrary.Map_Clear` (`self.tiles`)))

(fn `CalcCircularTilePos`
  (params (GridPos :type "/Game/Jamie/Structs/Struct_GridPosition Structure"))
  (returns (`World Position` :type "Vector Structure"))
  (locals (offset :type "Float (double-precision)"))
  (bind _nodesize_x (`KismetMathLibrary.BreakVector` (`self.nodeSize`)))
  (bind (_nodesize_x_2 _nodesize_y) (`KismetMathLibrary.BreakVector` (`self.nodeSize`)))
  (bind _nodesize_x_3 (`KismetMathLibrary.BreakVector` (`self.nodeSize`)))
  (bind (_gridpos_x _gridpos_y) (break `/Game/Jamie/Structs/Struct_GridPosition` (`local.GridPos`)))
  ;[1 1 1] Calculates the offset by adding an offset on the X each row will have a larger offset giving a circular appearence
  (set `local.offset` (* _gridpos_y _nodesize_x_3)) ; Offset = gridpos.y * nodeSize.x
  (return (`KismetMathLibrary.MakeVector` (+ (* GridPos_x_2_1255F2194F7E6F41CE9C6683B084C841 (* _nodesize_x 2.0)) (`local.offset`)) (* (* GridPos_Y_4_650A3D80459B33B480625A99FAB7EBAC (* _nodesize_y 2.0)) 0.75))) ; Return node position
)

(fn `CalcSquareTilePos`
  (params (GridPosition :type "/Game/Jamie/Structs/Struct_GridPosition Structure"))
  (returns (Position :type "Vector Structure"))
  (locals (offset :type "Float (double-precision)"))
  (bind _nodesize_x (`KismetMathLibrary.BreakVector` (`self.nodeSize`)))
  (bind (_nodesize_x_2 _nodesize_y) (`KismetMathLibrary.BreakVector` (`self.nodeSize`)))
  (bind _nodesize_x_3 (`KismetMathLibrary.BreakVector` (`self.nodeSize`)))
  (if (!= (mod GridPosition_Y_4_650A3D80459B33B480625A99FAB7EBAC 2) 0)
    ;[1 1 1] Add an offset to the X if the Y is odd
    (set `local.offset` (/ (* _nodesize_x_3 2.0) 2.0)))
  (return (`KismetMathLibrary.MakeVector` (+ (* GridPosition_x_2_1255F2194F7E6F41CE9C6683B084C841 (* _nodesize_x 2.0)) (`local.offset`)) (* (* GridPosition_Y_4_650A3D80459B33B480625A99FAB7EBAC (* _nodesize_y 2.0)) 0.75))))

(fn `GenrateCircularGrid`
  (bind _radius (`self.radius`))
  (bind _nodesize_x (`KismetMathLibrary.BreakVector` (`self.nodeSize`)))
  (bind _radius_2 (`self.radius`))
  (`|ExecutionSequence`
    (:`then_0`
      ;[1 1 1] Foward half of circle
      (for _index (range (+ (- _radius_2 (/ _radius_2 2)) 1))
        (for _index_2 (range (+ (- (`self.radius`) _index) 1))
          (`self.SpawnNode` (`self.CalcCircularTilePos` (make `/Game/Jamie/Structs/Struct_GridPosition` _index_2 _index)) (make `/Game/Jamie/Structs/Struct_GridPosition` _index_2 _index)))))
    (:`then_1`
      ;[1 1 1] Backward half of circle
      (for _index_3 (range 1 (+ (- _radius (/ _radius 2)) 1))
        (for _index_4 (range (+ (- (`self.radius`) _index_3) 1))
          (bind _returnvalue (* _index_4 -1))
          (bind _returnvalue_2 (* _index_3 -1))
          (`self.SpawnNode` (+ (`self.CalcCircularTilePos` (make `/Game/Jamie/Structs/Struct_GridPosition` _returnvalue _returnvalue_2)) (`KismetMathLibrary.MakeVector` (* _nodesize_x (* (`KismetMathLibrary.Conv_IntToDouble` (`self.radius`)) 2.0)))) (make `/Game/Jamie/Structs/Struct_GridPosition` _returnvalue _returnvalue_2)))))))

(fn `GenrateSquareGrid`
  (bind (_griddimentions_x _griddimentions_y) (break `/Game/Jamie/Structs/Struct_GridPosition` (`self.gridDimentions`)))
  ;[1 1 1] Loop Through grid
  (for _index (range _griddimentions_x)
    (for _index_2 (range _griddimentions_y)
      (`self.SpawnNode` (`self.CalcSquareTilePos` (make `/Game/Jamie/Structs/Struct_GridPosition` _index _index_2)) (make `/Game/Jamie/Structs/Struct_GridPosition` _index _index_2)))))

(fn `GetNodeDimentions`
  (bind _node (`self.SpawnNode` (0.0 0.0 0.0)))
  (set `self.nodeSize` (`.BoxExtent` (`self.GetActorBounds` _node true false)))
  (`self.K2_DestroyActor` _node)
  (`BlueprintMapLibrary.Map_Clear` (`self.tiles`)))

(fn `SpawnNode`
  (params (WorldPosition :type "Vector Structure") (`Grid Pos` :type "/Game/Jamie/Structs/Struct_GridPosition Structure"))
  (returns (Node :type "Actor Object Reference"))
  (bind _returnvalue (`|SpawnActorFromClass` (`self.node`) (`KismetMathLibrary.MakeTransform` WorldPosition (struct :`Yaw` 90.0)) "Undefined" "OverrideRootScale" null null))
  (`BlueprintMapLibrary.Map_Add` (`self.tiles`) `Grid Pos` _returnvalue)
  (`self.K2_AttachToActor` _returnvalue self "None" "KeepRelative" "KeepRelative" "KeepRelative" true)
  (return _returnvalue))

(fn `UserConstructionScript`)