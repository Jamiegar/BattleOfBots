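; Actor component that pre-spawns and reuses actors through an object pool keyed by class.
; On BeginPlay it spawns each configured class at the owner's location, deactivates the instances and sends them InitMessage.
; Spawn requests pop the last free instance, position and activate it, or print an error without growing the pool.
; Recycling returns actors to their class array and disables collision, visibility and tick.
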(event `self.ReceiveBeginPlay`
  (`self.SetUpPool`))

(fn `RecycleActorInPool`
  (params (Actor :type "Actor Object Reference"))
  (locals (classType :type "Actor Class Reference"))
  (bind _actor (`local.Actor`))
  (bind (_value _returnvalue) (`BlueprintMapLibrary.Map_Find` (`self.Pool`) (`local.classType`)))
  (set `local.classType` (`GameplayStatics.GetObjectClass` Actor))
  (if _returnvalue
    (`KismetArrayLibrary.Array_Add` (`.Obj_3_748C714041CBB6143D241B83B7749390` (break `/Game/Jamie/Blueprint/Components/Struct_ObjectPool` _value)) _actor)
    (`self.SetActorActive` _actor)
    (else
      (`KismetSystemLibrary.PrintString` "Type not in pool"))))

(fn `SetUpPool`
  (locals (spawnedActors :type "Array of Actor Object Reference") (actorToSpawn :type "Actor Class Reference"))
  (for _array_element (`self.InitalPool`)
    (bind (_object _number) (break `/Game/Jamie/Blueprint/Components/Struct_PoolObject` _array_element))
    (set `local.actorToSpawn` _object) ; Set Local Actor
    (if (not (`BlueprintMapLibrary.Map_Contains` (`self.Pool`) _object))
      (for _ (range 1 (+ _number 1))
        ;[1 1 1] Spawn Actor
        (bind _returnvalue (`|SpawnActorFromClass` (`local.actorToSpawn`) (`KismetMathLibrary.MakeTransform` (`Actor.K2_GetActorLocation` (`self.GetOwner`))) "Undefined" "OverrideRootScale" null null))
        (`KismetArrayLibrary.Array_Add` (`local.spawnedActors`) _returnvalue) ; Store in local array
        (`self.SetActorActive` _returnvalue
          (:`Finish`
            (message `/Game/Jamie/Interfaces/GameMode/BPI_Initalize.Init` _returnvalue))))
      (`BlueprintMapLibrary.Map_Add` (`self.Pool`) (`local.actorToSpawn`) (make `/Game/Jamie/Blueprint/Components/Struct_ObjectPool` (`local.spawnedActors`))) ; Add to array
      (`KismetArrayLibrary.Array_Clear` (`local.spawnedActors`)) ; Clear local array once added to pool
    )))

(fn `SpawnActorFromPool`
  (params (ActorToSpawn :type "Actor Class Reference") (`Transform Spawn` :type "Transform Structure"))
  (returns (`Actor Reference` :type "Actor Object Reference"))
  (locals (actor :type "Actor Object Reference"))
  (bind (_value _returnvalue) (`BlueprintMapLibrary.Map_Find` (`self.Pool`) ActorToSpawn))
  (bind _obj (break `/Game/Jamie/Blueprint/Components/Struct_ObjectPool` _value))
  (bind _returnvalue_2 (`KismetArrayLibrary.Array_LastIndex` _obj))
  (if _returnvalue
    (if (`KismetArrayLibrary.Array_IsValidIndex` _obj _returnvalue_2)
      (set `local.actor` (`|GetArrayItem` _obj _returnvalue_2)) ; Set Local ref to found Actor
      (`KismetArrayLibrary.Array_Remove` _obj _returnvalue_2) ; Remove from array so it is not used\nwhile it is active
      (`Actor.K2_SetActorTransform` (`local.actor`) (`local.Transform Spawn`) false false) ; Set actor tranform on Spawn
      (`self.SetActorActive` (`local.actor`) true
        (:`Finish`
          (return (`local.actor`))))
      (else
        (`KismetSystemLibrary.PrintString` "No Items left in pool (Not valid index)" true true (struct :`R` 1.0 :`G` 0.021375 :`A` 1.0))))
    (else
      (`KismetSystemLibrary.PrintString` "Object not in pool"))))