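; Component that lets a character wear and cycle through hat cosmetics.
; On init it loads row names from D_Cosmetics and spawns a BP_Cosmetic actor attached to the mesh's CATRigHatPoint socket.
; Next and Previous step a wrapping index into those rows to apply the mesh, though Previous only applies it when wrapping.
; SetCosmetic applies a given name and mesh directly, without updating the index.
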(event `Init Cosmetic Component`
  (params (CharcterMesh :type "SkeletalMeshComponent Object Reference"))
  ;[1 1 1] Initalisation
  (set `self.CharcterMesh` CharcterMesh)
  (bind _outrownames (`DataTableFunctionLibrary.GetDataTableRowNames` "/Game/Jamie/DataTables/D_Cosmetics.D_Cosmetics"))
  (set `self.AllCosmetics` _outrownames)
  (bind _returnvalue (`|SpawnActorFromClass` "/Game/Jamie/Blueprint/Characters/BP_Cosmetic.BP_Cosmetic_C" (`KismetMathLibrary.MakeTransform` (0.0 0.0 0.0)) "Undefined" "OverrideRootScale" (`self.GetOwner`) null))
  (bind _output_get (set `self.CosmeticSlot` _returnvalue))
  (`Actor.K2_AttachToComponent` _output_get (`self.CharcterMesh`) "CATRigHatPoint" "KeepRelative" "KeepWorld" "KeepWorld" true))

(event `NextCharcterCosmetic`
  ;[1 1 1] Next Hat
  (bind _result (`/Engine/EditorBlueprintResources/StandardMacros.IncrementInt` (`self.cosmeticIndex`))
    (:`  `
      (if (> _result (- (`KismetArrayLibrary.Array_Length` (`self.AllCosmetics`)) 1))
        (set `self.cosmeticIndex` 0))
      (`self.SetCosmeticMeshFromData`))))

(event `PreviousCharcterCosmetic`
  ;[1 1 1] Previous Hat
  (bind _result (`/Engine/EditorBlueprintResources/StandardMacros.DecrementInt` (`self.cosmeticIndex`))
    (:`  `
      (if (< _result 0)
        (set `self.cosmeticIndex` (- (`KismetArrayLibrary.Array_Length` (`self.AllCosmetics`)) 1))
        (`self.SetCosmeticMeshFromData`)))))

(event `SetCosmetic`
  (params (CosmeticName :type String) (Cosmetic :type "StaticMesh Object Reference"))
  (set `self.currentCosmeticName` CosmeticName)
  (bind _output_get (set `self.currentCosmetic` Cosmetic))
  (`/Game/Jamie/Blueprint/Characters/BP_Cosmetic.Set Cosmetic Mesh` (`self.CosmeticSlot`) _output_get))

(fn `SetCosmeticMeshFromData`
  (bind _returnvalue (`|GetDataTableRow` "/Game/Jamie/DataTables/D_Cosmetics.D_Cosmetics" (`|GetArrayItem` (`self.AllCosmetics`) (`self.cosmeticIndex`)))
    (:`then`
      (bind (_name _mesh) (break `/Game/Jamie/Structs/StructsForDataTables/Struct_CustomHats` _returnvalue))
      (set `self.currentCosmeticName` _name)
      (bind _output_get (set `self.currentCosmetic` _mesh))
      (`/Game/Jamie/Blueprint/Characters/BP_Cosmetic.Set Cosmetic Mesh` (`self.CosmeticSlot`) _output_get))))