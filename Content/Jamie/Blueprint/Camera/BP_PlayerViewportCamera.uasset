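; Shared multi-character viewport camera that frames the game mode's characters, or returns to its starting position, depending on camera state.
; Each tick it lerps the sphere toward the average location of characters above minimum Z, and spring arm length toward their largest pairwise distance, both clamped.
; With fewer than two in range, separate transition speeds apply.
; Bound events play world camera shakes, with Mid and Long assets crossed.
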(event `/Game/Jamie/Interfaces/GameMode/BPI_Initalize.Init`
  (bind _currentgamemode (message `/Game/Jamie/Interfaces/GameMode/BPI_GameMode.GetGameMode` (`GameplayStatics.GetGameMode`)))
  (set `self.characters` (`/Game/Jamie/Blueprint/GameMode/GM_Base_BrawlOfBots.character` _currentgamemode))
  ;[1 1 1] Save starting position
  (set `self.defaultPosition` (`SceneComponent.K2_GetComponentLocation` (`self.Sphere`)))
  (set `self.defaultSpringArm` (`SpringArmComponent.TargetArmLength` (`self.SpringArm`)))
  (set `self.hasInitalized` true))

(event `self.ReceiveTick`
  (params (DeltaSeconds :type "Float (single-precision)"))
  (if (`self.hasInitalized`)
    (`self.RunCameraState`)))

(event `Camera Shake Quick ED_Event`
  ;[0.6414 0.4225 1] Camera Shake ED
  (`GameplayStatics.PlayWorldCameraShake` "/Game/Callum/BP/Camera/CameraShakes/CameraShake_Quick.CameraShake_Quick_C" (`self.K2_GetActorLocation`) 0.0 10000000.0 1.0 true))

(event `self.ReceiveBeginPlay`
  ;[0.6414 0.4225 1] Camera Shake ED
  (`|ExecutionSequence`
    (:`then_0`
      (add `self.Camera Shake Quick ED` (delegate `Camera Shake Quick ED_Event`)))
    (:`then_1`
      (add `self.Camera Shake Long ED` (delegate `Camera Shake Long ED_Event`)))
    (:`then_2`
      (add `self.Camera Shake Mid ED` (delegate `Camera Shake Mid ED_Event`)))))

(event `Camera Shake Long ED_Event`
  ;[0.6414 0.4225 1] Camera Shake ED
  (`GameplayStatics.PlayWorldCameraShake` "/Game/Callum/BP/Camera/CameraShakes/CameraShake_Mid.CameraShake_Mid_C" (`self.K2_GetActorLocation`) 0.0 10000000.0 1.0 true))

(event `Camera Shake Mid ED_Event`
  ;[0.6414 0.4225 1] Camera Shake ED
  (`GameplayStatics.PlayWorldCameraShake` "/Game/Callum/BP/Camera/CameraShakes/CameraShake_Long.CameraShake_Long_C" (`self.K2_GetActorLocation`) 0.0 10000000.0 1.0 true))

(fn `Calc Sprin Arm Length for Characters`
  (locals (currentPlayer :type "Actor Object Reference") (distance :type "Array of Float (double-precision)") (charactersInRange :type "Array of Actor Object Reference"))
  (bind _output_get (set `local.charactersInRange` (`self.GetCharactersInRange`)))
  (for _array_element _output_get
    (set `local.currentPlayer` _array_element)
    ;[1 1 1] Create array of distances between each character
    (for _index (range (`KismetArrayLibrary.Array_Length` (`local.charactersInRange`)))
      (`KismetArrayLibrary.Array_Add` (`local.distance`) (`self.GetDistanceTo` (`local.currentPlayer`) (`|GetArrayItem` (`local.charactersInRange`) _index)))))
  ;[1 1 1] Lerp Arm length to max distance
  (`self.SetTargetArmLength` (`.MaxValue` (`KismetMathLibrary.MaxOfFloatArray` (`local.distance`))))
  (`KismetArrayLibrary.Array_Clear` (`local.distance`)))

(fn `CalcCamreaMovement`
  (params (Location :type "Vector Structure"))
  ;[1 1 1] Set world position of sphere
  (`SceneComponent.K2_SetWorldLocation` (`self.Sphere`) (`KismetMathLibrary.VLerp` (`SceneComponent.K2_GetComponentLocation` (`self.Sphere`)) (`KismetMathLibrary.MakeVector` (.x Location) (.y Location) (`KismetMathLibrary.FClamp` (.z Location) (`self.minCameraZ`) (`self.MaxCameraZ`))) (select `bool` (< (`KismetArrayLibrary.Array_Length` (`self.GetCharactersInRange`)) 2) :`false` (`self.cameraMoveSpeed`) :`true` (`self.transitionMovementSpeed`))) false false))

(fn `GetCharactersInRange`
  (returns (InRangeActors :type "Array of Actor Object Reference"))
  (locals (InRangeCharacters :type "Array of Actor Object Reference") (currentIndex :type "Actor Object Reference"))
  (for _array_element (`self.characters`)
    (bind _output_get (set `local.currentIndex` _array_element))
    (if (> (.z (`self.K2_GetActorLocation` _output_get)) (`self.minCameraZ`))
      (`KismetArrayLibrary.Array_Add` (`local.InRangeCharacters`) (`local.currentIndex`))))
  (return (`local.InRangeCharacters`)))

(fn `RunCameraState`
  (switch `/Game/Jamie/Enum/Enum_CameraStates` (`self.CameraState`)
    (:`NewEnumerator0`
      ;[1 1 1] Camera follows character average point
      (bind _returnvalue (`GameplayStatics.GetActorArrayAverageLocation` (`self.GetCharactersInRange`)))
      (`self.CalcCamreaMovement` _returnvalue)
      (`self.Calc Sprin Arm Length for Characters`))
    (:`NewEnumerator1`
      ;[1 1 1] Sets camera back to its inital position
      (`self.CalcCamreaMovement` (`self.defaultPosition`))
      (`self.SetTargetArmLength` (`self.defaultSpringArm`)))))

(fn `SetTargetArmLength`
  (params (ArmLength :type "Float (double-precision)"))
  (set `SpringArmComponent.TargetArmLength` (`KismetMathLibrary.FClamp` (`KismetMathLibrary.Lerp` (`SpringArmComponent.TargetArmLength` (`self.SpringArm`)) ArmLength (select `bool` (< (`KismetArrayLibrary.Array_Length` (`self.GetCharactersInRange`)) 2) :`false` (`self.cameraZoomSpeed`) :`true` (`self.transitionZoomSpeed`))) (`self.minCameraDistance`) (`self.maxCameraDistance`)) (`self.SpringArm`)))

(fn `UserConstructionScript`)