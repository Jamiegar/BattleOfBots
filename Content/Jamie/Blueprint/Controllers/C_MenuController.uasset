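; Menu player controller that provides a gamepad-driven virtual mouse cursor in place of the system cursor.
; Init spawns the cursor widget; left-stick input past a dead zone moves it, clamped to screen resolution.
; Tick positions the cursor, line-traces from its viewport-scaled, deprojected position, and feeds the hit to a WidgetInteraction component as a custom hit result.
; The Jump action acts as left click on that component.
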(event `/Game/Jamie/Interfaces/GameMode/BPI_Initalize.Init`
  ;[1 0.9007 0.1567] Initalisation
  ;;[1 1 1] Create virtual mouse widget and add to viewport
  (bind _returnvalue (`|CreateWidget` "/Game/Jamie/UI/UI_ControllerMouse.UI_ControllerMouse_C" self))
  (bind _output_get (set `self.VirtualMouse` _returnvalue))
  (`UserWidget.AddToViewport` _output_get 0)
  (set `self.bShowMouseCursor` false) ; Set mouse cursor to be off
  ;;[1 1 1] Set starting position
  (set `self.NewPositionX` 960.0)
  (set `self.NewPositionY` 400.0)
  (add `self.OnDestroyed` (`|CreateDelegate` :!event `DestroyVirtualMouse`)))

(event `self.ReceiveTick`
  (params (DeltaSeconds :type "Float (single-precision)"))
  (bind _rendertransform_translation (break `WidgetTransform` (`Widget.RenderTransform` (`/Game/Jamie/UI/UI_ControllerMouse.Mouse` (`self.VirtualMouse`)))))
  (bind (_worldposition _worlddirection) (`GameplayStatics.DeprojectScreenToWorld` self (* _rendertransform_translation (`WidgetLayoutLibrary.GetViewportScale`))))
  ;[0.609 1 0.202] Tick
  (`/Engine/EditorBlueprintResources/StandardMacros.IsValid` (`self.VirtualMouse`) ; Valid Check
    (:`Is Valid`
      ;;[1 1 1] Set new position of virtual mouse
      (`Widget.SetRenderTranslation` (`/Game/Jamie/UI/UI_ControllerMouse.Mouse` (`self.VirtualMouse`)) (`KismetMathLibrary.MakeVector2D` (`self.NewPositionX`) (`self.NewPositionY`)))
      ;;[1 1 1] Fire line trace out from virtual mouse
      (bind _outhit (`KismetSystemLibrary.LineTraceSingle` _worldposition (+ _worldposition (* _worlddirection 100000.0)) "TraceTypeQuery1" false (`|MakeArray` self :!type "Actor Object Reference")))
      ;;[1 1 1] Set custom hit result for widget interaction
      (`WidgetInteractionComponent.SetCustomHitResult` (`self.WidgetInteraction`) _outhit))))

(event `InputAction|Jump`
  (params (Key :type "Key Structure"))
  (bind _widgetinteraction (`self.WidgetInteraction`))
  ;[1 1 1] Interaction key pressed
  (:`Pressed`
    (`WidgetInteractionComponent.PressPointerKey` _widgetinteraction "LeftMouseButton"))
  (:`Released`
    (`WidgetInteractionComponent.ReleasePointerKey` _widgetinteraction "LeftMouseButton")))

(event `InputAxis|MenuLeftStickX`
  (params (AxisValue :type "Float (single-precision)"))
  (bind _screenresolution_x (break `IntPoint` (`self.ScreenResolution`)))
  (bind (_screenresolution_x_2 _screenresolution_y) (break `IntPoint` (`self.ScreenResolution`)))
  (bind _rendertransform (`Widget.RenderTransform` (`/Game/Jamie/UI/UI_ControllerMouse.Mouse` (`self.VirtualMouse`))))
  ;[0.3 0.8208 1] Controller Input Axis
  (bind _output_get (set `self.LeftStickX` AxisValue))
  (if (> (`KismetMathLibrary.Abs` _output_get) 0.1)
    ;[0.1587 0.3 1] Calculate the new position of the virtural mouse
    (`/Engine/EditorBlueprintResources/StandardMacros.IsValid` (`self.VirtualMouse`) :!label _label ; Check the virtual Mouse is valid
      (:`Is Valid`
        (bind _returnvalue (`GameUserSettings.GetGameUserSettings`))
        (set `self.ScreenResolution` (`GameUserSettings.GetScreenResolution` _returnvalue))
        ;;[1 1 1] Clamp The new position to the screen resolution so that the virtual mouse does not go outside the screen
        (set `self.NewPositionX` (`KismetMathLibrary.FClamp` (+ (`KismetMathLibrary.BreakVector2D` (break `WidgetTransform` _rendertransform)) (* (`self.VirtualMouseSpeed`) (`self.LeftStickX`) (`GameplayStatics.GetWorldDeltaSeconds`))) 0.0 (`KismetMathLibrary.Conv_IntToDouble` _screenresolution_x)))
        (set `self.NewPositionY` (`KismetMathLibrary.FClamp` (+ (`.Y` (`KismetMathLibrary.BreakVector2D` (break `WidgetTransform` _rendertransform))) (* (`self.VirtualMouseSpeed`) (`self.LeftStickY`) (`GameplayStatics.GetWorldDeltaSeconds`))) 0.0 (`KismetMathLibrary.Conv_IntToDouble` _screenresolution_y)))))))

(event `InputAxis|MenuLeftStickY`
  (params (AxisValue :type "Float (single-precision)"))
  ;[0.3 0.8208 1] Controller Input Axis
  (bind _output_get (set `self.LeftStickY` AxisValue))
  (if (> (`KismetMathLibrary.Abs` _output_get) 0.1)
    (goto _label)))

(fn `DestroyVirtualMouse`
  (params (DestroyedActor :type "Actor Object Reference"))
  (bind _virtualmouse (`self.VirtualMouse`))
  (`/Engine/EditorBlueprintResources/StandardMacros.IsValid` _virtualmouse
    (:`Is Valid`
      (`Widget.RemoveFromParent` _virtualmouse))))

(fn `UserConstructionScript`)