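; Game mode for the win screen that presents the winning player's character in a victory pose.
; A state switch runs Setup, which spawns a bot character at the first spawn point, applies the winner's hat cosmetic from the game instance, and enables UI input with a mouse cursor.
; Setup then advances to PreGame, which flags spawned characters as in their win state; InGame and PostGame are empty.
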(event `self.ReceiveBeginPlay`
  (bind _instance (message `/Game/Jamie/Interfaces/GameInstance/BPI_GameInstance.GetInstance` (`GameplayStatics.GetGameInstance`)))
  (set `self.GameInstance` _instance)
  (`self.SwitchGameState` "NewEnumerator0"))

(event `Setup`
  (bind _returnvalue (`GameplayStatics.GetPlayerController` 0))
  (`self.GetPlayerStarts`)
  (`self.SpawnCharcter`)
  (message `/Game/Jamie/Interfaces/GameMode/BPI_Initalize.Init` _returnvalue)
  (`WidgetBlueprintLibrary.SetInputMode_GameAndUIEx` _returnvalue null)
  (set `PlayerController.bShowMouseCursor` true _returnvalue)
  (`self.SwitchGameState` "NewEnumerator1"))

(event `PreGame`
  (`self.SetCharacterWinPose`))

(event `InGame`)

(event `PostGame`)

(fn `GetPlayerStarts`
  (bind _outactors (`GameplayStatics.GetAllActorsOfClass` "/Game/Jamie/Blueprint/Characters/BP_SpawnPoint.BP_SpawnPoint_C")) ; Gets all the spawners in the world
  (set `self.characterSpawnPoints` _outactors) ; Set a variable to that array of objects
)

(fn `SetCharacterWinPose`
  (for _array_element (`self.Characters`)
    (bind _character (message `/Game/Jamie/Interfaces/Character/BPI_Character.GetCharacter` _array_element))
    (set `/Game/Callum/Characters/BP_BotCharacter.InWinState` true _character)))

(fn `SpawnCharcter`
  (bind _returnvalue (`|SpawnActorFromClass` "/Game/Callum/Characters/BP_BotCharacter.BP_BotCharacter_C" (`self.GetTransform` (`|GetArrayItem` (`self.characterSpawnPoints`))) "Undefined" "OverrideRootScale" null null))
  (`KismetArrayLibrary.Array_Add` (`self.Characters`) _returnvalue)
  (message `/Game/Jamie/Interfaces/GameMode/BPI_Initalize.Init` _returnvalue)
  (bind _character (message `/Game/Jamie/Interfaces/Character/BPI_Character.GetCharacter` _returnvalue))
  (`/Game/Jamie/Blueprint/Components/Com_HatCosmetic.SetCosmetic` (`/Game/Callum/Characters/BP_BotCharacter.Com_HatCosmetic` _character) (`/Game/Jamie/Blueprint/Managers/BP_BrawlOfBots_Instance.winnigPlayerCosmetic` (`self.GameInstance`))))

(fn `SwitchGameState`
  (params (`New Game State` :type "/Game/Jamie/Enum/GameMode/Enum_GameStates Enum" :default "NewEnumerator0"))
  (bind _output_get (set `self.CurrentGameState` `New Game State`))
  (switch `/Game/Jamie/Enum/GameMode/Enum_GameStates` _output_get
    (:`NewEnumerator0`
      (`self.Setup`))
    (:`NewEnumerator1`
      (`self.PreGame`))
    (:`NewEnumerator2`
      (`self.InGame`))
    (:`NewEnumerator3`
      (`self.PostGame`))))

(fn `UserConstructionScript`)