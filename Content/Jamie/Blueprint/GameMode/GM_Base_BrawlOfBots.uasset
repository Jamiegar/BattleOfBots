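; Base game mode for Brawl of Bots, a local multiplayer match that runs through Setup, PreGame, InGame and PostGame states.
; Setup initializes map, power-up and lives managers, creates local controllers and spawns characters at spawn points.
; InGame possesses characters, shares the map manager's camera and starts the hazard timer.
; Also toggles the pause menu; hazard functions are placeholders for child modes, and PostGame is empty and unreached.
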(event `self.ReceiveBeginPlay`
  (`self.SwitchGameState` "NewEnumerator0"))

(event `Game Setup`
  (`self.SetupMapManager`)
  (`self.SetupPowerUPManager`)
  (`self.SetupLivesManager`)
  (`self.GetPlayerStarts`)
  (`self.CreateControllers` (`self.numberOfPlayers`))
  (`self.Spawn Players`)
  (`self.SetupMapHazard`)
  (`self.SwitchGameState` "NewEnumerator1"))

(event `PreGame`
  (`/Game/Jamie/Blueprint/Managers/BP_BaseMapManager.InitalizeCamera` (`self.mapManager`))
  (`self.SwitchGameState` "NewEnumerator2"))

(event `InGame`
  ;[1 1 1] Game starts
  (`self.PossessCharacters`)
  (`self.CountDownToMapHazard`))

(event `PostGame`
  ;[1 1 1] Clean up
)

(fn `ActivateMapHazard`
  (`KismetSystemLibrary.PrintString` "No Map Hazard" true true (struct :`R` 1.0 :`B` 0.004321 :`A` 1.0) 5.0))

(fn `CountDownToMapHazard`
  (`KismetSystemLibrary.K2_SetTimerDelegate` (`|CreateDelegate` :!event `ActivateMapHazard`) (`self.mapHazardTimer`)))

(fn `CreateControllers`
  (params (NumberOfControllers :type Integer))
  ;[1 1 1] Removes the default controller created
  (`GameplayStatics.RemovePlayer` (`GameplayStatics.GetPlayerController` 0))
  (for _ (range NumberOfControllers)
    (bind _returnvalue (`GameplayStatics.CreatePlayer` -1))
    (`KismetArrayLibrary.Array_Add` (`self.controllers`) _returnvalue) ; Add the controller to an array of controllers
    (message `/Game/Jamie/Interfaces/GameMode/BPI_Initalize.Init` _returnvalue)))

(fn `GetGameMode`
  (returns (CurrentGameMode :type "/Game/Jamie/Blueprint/GameMode/GM_Base_BrawlOfBots Object Reference"))
  (return self))

(fn `GetPlayerStarts`
  (bind _outactors (`GameplayStatics.GetAllActorsOfClass` "/Game/Jamie/Blueprint/Characters/BP_SpawnPoint.BP_SpawnPoint_C")) ; Gets all the spawners in the world
  (set `self.characterSpawnPoints` _outactors) ; Set a variable to that array of objects
)

(fn `GetPowerUpManger`
  (returns (PowerUPManager :type "/Game/Jamie/Blueprint/Managers/BP_PowerupManager Object Reference"))
  (return (`self.powerUpManager`)))

(fn `PossessCharacters`
  ;[1 1 1] For each controllers possess the charcter with the same index
  (for (_array_element _array_index) (`self.controllers`)
    (bind _character (message `/Game/Jamie/Interfaces/Character/BPI_Character.GetCharacter` (`|GetArrayItem` (`self.character`) _array_index))) ; Gets direct refrence to character
    (`Controller.Possess` _array_element _character)
    ;[1 1 1] Set the view target to be the camrea in the world
    (`PlayerController.SetViewTargetWithBlend` _array_element (`/Game/Jamie/Blueprint/Managers/BP_BaseMapManager.camrea` (`self.mapManager`)) 0.1 "VTBlend_Linear" 0.0 false)))

(fn `SetupLivesManager`
  (bind _returnvalue (`GameplayStatics.GetActorOfClass` "/Game/Callum/BP/Managers/BP_lives_manager.BP_lives_manager_C"))
  (bind _output_get (set `self.livesManager` _returnvalue))
  (message `/Game/Jamie/Interfaces/GameMode/BPI_Initalize.Init` _output_get))

(fn `SetupMapHazard`
  (`KismetSystemLibrary.PrintString` "/////////////////////////////////////////////////////// \nNo Map Hazard Set up (Set Up In child GameMode)  \n///////////////////////////////////////////////////////" true true (struct :`R` 1.0 :`B` 0.004321 :`A` 1.0) 5.0))

(fn `SetupMapManager`
  (bind _returnvalue (`GameplayStatics.GetActorOfClass` "/Game/Jamie/Blueprint/Managers/BP_BaseMapManager.BP_BaseMapManager_C"))
  (`/Engine/EditorBlueprintResources/StandardMacros.IsValid` _returnvalue
    (:`Is Valid`
      (bind _output_get (set `self.mapManager` _returnvalue))
      (message `/Game/Jamie/Interfaces/GameMode/BPI_Initalize.Init` _output_get))
    (:`Is Not Valid`
      (`KismetSystemLibrary.PrintString` "Place Map Manager in world"))))

(fn `SetupPowerUPManager`
  ;[1 1 1] Find if there is a Power-up manger already in the scene
  (bind _returnvalue (`GameplayStatics.GetActorOfClass` "/Game/Jamie/Blueprint/Managers/BP_PowerupManager.BP_PowerupManager_C"))
  (bind _output_get (set `self.powerUpManager` _returnvalue))
  (`/Engine/EditorBlueprintResources/StandardMacros.IsValid` _output_get
    (:`Is Valid`
      ;[1 1 1] If it is already placed in the world then initalize it
      (message `/Game/Jamie/Interfaces/GameMode/BPI_Initalize.Init` (`self.powerUpManager`)))
    (:`Is Not Valid`
      ;[1 1 1] If there is not one in the scene then create the manager and initalize it
      (bind _returnvalue_2 (`|SpawnActorFromClass` "/Game/Jamie/Blueprint/Managers/BP_PowerupManager.BP_PowerupManager_C" (`KismetMathLibrary.MakeTransform` (0.0 0.0 0.0)) "Undefined" "OverrideRootScale" null null))
      (bind _output_get_2 (set `self.powerUpManager` _returnvalue_2))
      (message `/Game/Jamie/Interfaces/GameMode/BPI_Initalize.Init` _output_get_2))))

(fn `Spawn Players`
  (for _index (range (`self.numberOfPlayers`))
    (bind _returnvalue (`|SpawnActorFromClass` (`self.playerCharacters`) (`self.GetTransform` (`|GetArrayItem` (`self.characterSpawnPoints`) _index)) "Undefined" "OverrideRootScale" null null)) ; Spawn the character at the player start transform
    (`KismetArrayLibrary.Array_Add` (`self.character`) _returnvalue) ; Add character to array of all the characters spawned in the game
  ))

(fn `SwitchGameState`
  (params (`Change State` :type "/Game/Jamie/Enum/GameMode/Enum_GameStates Enum" :default "NewEnumerator0"))
  (bind _output_get (set `self.currentGameState` `Change State`)) ; Set the current state to be the one that it has been changed to
  ;[1 1 1] Switch on the change to run the appropriate event
  (switch `/Game/Jamie/Enum/GameMode/Enum_GameStates` _output_get
    (:`NewEnumerator0`
      (`self.Game Setup`))
    (:`NewEnumerator1`
      (`self.PreGame`))
    (:`NewEnumerator2`
      (`self.InGame`))
    (:`NewEnumerator3`
      (`self.PostGame`))))

(fn `TogglePause`
  (returns (IsGamePaused :type Boolean))
  (bind _output (`|GetArrayItem` (`self.controllers`)))
  (bind _output_2 (`|GetArrayItem` (`self.controllers`)))
  ;[1 1 1] Because we want to toggle pause the branch does the opposite. e.g. if isGamePaused == true then unpause game
  (if (`self.isGamePaused`)
    (bind _returnvalue (`GameplayStatics.SetGamePaused` false))
    (set `self.isGamePaused` _returnvalue)
    (`Widget.RemoveFromParent` (`self.pauseMenu`))
    (`WidgetBlueprintLibrary.SetInputMode_GameOnly` _output)
    (set `PlayerController.bShowMouseCursor` false _output)
    (return false)
    (else
      (bind _returnvalue_2 (`GameplayStatics.SetGamePaused` true))
      (set `self.isGamePaused` _returnvalue_2)
      (`/Engine/EditorBlueprintResources/StandardMacros.IsValid` (`self.pauseMenu`)
        (:`Is Valid`
          (`UserWidget.AddToViewport` (`self.pauseMenu`) 0))
        (:`Is Not Valid`
          (bind _returnvalue_3 (`|CreateWidget` "/Game/Jamie/UI/MainMenu/UI_PauseMenu.UI_PauseMenu_C"))
          (bind _output_get (set `self.pauseMenu` _returnvalue_3))
          (`UserWidget.AddToViewport` _output_get 0)))
      (`WidgetBlueprintLibrary.SetInputMode_GameAndUIEx` _output_2 null)
      (set `PlayerController.bShowMouseCursor` true _output_2))))

(fn `UserConstructionScript`)