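; Game mode for a map with a spiked ball hazard, providing the hazard's setup and activation logic.
; SetupMapHazard spawns BP_SpikeyBall at the MapManager's hazard spawn point, offset by the manager's location, passes it the player character reference and freezes its physics.
; ActivateMapHazard re-enables physics on the ball and calls its InitMessage.
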(fn `ActivateMapHazard`
  (bind _spikeyballmaphazard (`self.spikeyBallMapHazard`))
  (`PrimitiveComponent.SetSimulatePhysics` (`/Game/Jamie/Blueprint/MapHazards/SpikeyBall/BP_SpikeyBall.Ball` _spikeyballmaphazard) true)
  (message `/Game/Jamie/Interfaces/GameMode/BPI_Initalize.Init` _spikeyballmaphazard))

(fn `SetupMapHazard`
  (bind _mapmanager (`self.mapManager`))
  (bind _returnvalue (`|SpawnActorFromClass` "/Game/Jamie/Blueprint/MapHazards/SpikeyBall/BP_SpikeyBall.BP_SpikeyBall_C" (`KismetMathLibrary.MakeTransform` (+ (`/Game/Jamie/Blueprint/Managers/BP_BattleMapManager.mapHazardSpawnPoint` _mapmanager) (`self.K2_GetActorLocation` _mapmanager))) "Undefined" "OverrideRootScale" null "NewEnumerator1" (`self.character`) null null))
  (bind _output_get (set `self.spikeyBallMapHazard` _returnvalue))
  (`PrimitiveComponent.SetSimulatePhysics` (`/Game/Jamie/Blueprint/MapHazards/SpikeyBall/BP_SpikeyBall.Ball` _output_get) false))

(fn `UserConstructionScript`
  (`parent.UserConstructionScript`))