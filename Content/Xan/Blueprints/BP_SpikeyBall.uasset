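; BP_SpikeyBall is a physics-driven hazard ball that repeatedly changes its roll direction after a start delay.
; ChangeRollType loops into one of two timed events, each zeroing velocity before applying a new impulse.
; Random mode biases each axis back toward the world origin, while player mode aims at a random Players entry, populated only with player 0.
; Hitbox overlap is placeholder detection that prints the hit actor, throttled by a resetting DoOnce.
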(event `self.ReceiveBeginPlay`
  ;[1 1 1] Begin Play
  (`|ExecutionSequence`
    (:`then_0`
      (`KismetArrayLibrary.Array_Add` (`self.Players`) (`GameplayStatics.GetPlayerCharacter` 0)))
    (:`then_1`
      (`KismetSystemLibrary.Delay` (`self.StartDelay`))
      (`self.Change Roll Type` (`self.DefaultRollType`)))))

(event `Random Direction`
  ;[1 1 1] Randomly sets an X & Y axis value and then rolls the ball using those values
  (`KismetSystemLibrary.Delay` (`self.ChangeDelay`))
  (`PrimitiveComponent.SetAllPhysicsLinearVelocity` (`self.Ball`) (0.0 0.0 0.0) false)
  (`self.ChangeAxisMovement` true)
  (`self.ChangeAxisMovement` false)
  (`self.Change Roll Type` (`self.DefaultRollType`)))

(event `Random Player Direction`
  ;[1 1 1] Randomly selects a player and then rolls the ball in their direction
  (`KismetSystemLibrary.RetriggerableDelay` (`self.ChangeDelay`))
  (bind _playertargeted (`self.TargetRandomPlayer` (`self.Players`)))
  (bind _output_get (set `self.Target` _playertargeted))
  (`PrimitiveComponent.SetAllPhysicsLinearVelocity` (`self.Ball`) (0.0 0.0 0.0) false)
  (`self.RollTowardTarget` _output_get)
  (`self.Change Roll Type` (`self.DefaultRollType`)))

(event `self.Hitbox.OnComponentBeginOverlap`
  (params (OverlappedComponent :type "PrimitiveComponent Object Reference") (OtherActor :type "Actor Object Reference") (OtherComp :type "PrimitiveComponent Object Reference") (OtherBodyIndex :type Integer) (bFromSweep :type Boolean) (SweepResult :type "HitResult Structure (by ref)"))
  ;[1 1 1] (placeholder hit detection)
  (`/Engine/EditorBlueprintResources/StandardMacros.DoOnce` false :!label _label
    (:`Completed`
      (`KismetSystemLibrary.PrintString` (`KismetTextLibrary.Conv_TextToString` (`|FormatText` "Spiky Ball hit {actor}" OtherActor)))
      (`KismetSystemLibrary.Delay` 1.0)
      (goto _label :!via `Reset`))))

(fn `Change Roll Type`
  (params (`Roll Type` :type "/Game/Xan/Enum/Enum_RollTypes Enum" :default "NewEnumerator0"))
  (switch `/Game/Xan/Enum/Enum_RollTypes` `Roll Type`
    (:`NewEnumerator0`
      (`self.Random Direction`))
    (:`NewEnumerator1`
      (`self.Random Player Direction`))))

(fn `ChangeAxisMovement`
  (params (`IsX?` :type Boolean))
  (locals (MinAxis :type "Float (double-precision)") (MaxAxis :type "Float (double-precision)") (AxisValue :type "Float (double-precision)" :default 1.0) (VectorValue :type "Vector Structure"))
  (bind _returnvalue (* (`KismetMathLibrary.RandomFloatInRange` (`local.MinAxis`) (`local.MaxAxis`)) (`self.RollTorque`)))
  (if `IsX?`
    (if (>= (.x (`SceneComponent.K2_GetComponentLocation` (`self.Ball`))) 0.0)
      (set `local.MinAxis` -1.0 :!label _label)
      (set `local.MaxAxis` 0.0)
      (else
        (set `local.MinAxis` 0.0 :!label _label_2)
        (set `local.MaxAxis` 1.0)))
    (elif (>= (.y (`SceneComponent.K2_GetComponentLocation` (`self.Ball`))) 0.0)
      (goto _label)
      (else
        (goto _label_2))))
  (if `IsX?`
    (bind _output_get (set `local.VectorValue` (`KismetMathLibrary.MakeVector` _returnvalue)))
    (else
      (set `local.VectorValue` (`KismetMathLibrary.MakeVector` 0.0 _returnvalue))))
  (`PrimitiveComponent.AddImpulse` (`self.Ball`) _output_get "None" false))

(fn `RollTowardTarget`
  (params (TargetActor :type "Actor Object Reference"))
  (if (`KismetSystemLibrary.IsValid` TargetActor)
    (`PrimitiveComponent.AddImpulse` (`self.Ball`) (* (`KismetMathLibrary.GetDirectionUnitVector` (`self.K2_GetActorLocation` self) (`self.K2_GetActorLocation` TargetActor)) (`self.RollTorque`)) "None" false)))

(fn `TargetRandomPlayer`
  (params (Players :type "Array of Actor Object Reference"))
  (returns (PlayerTargeted :type "Actor Object Reference"))
  (return (`|GetArrayItem` Players (`KismetMathLibrary.RandomIntegerInRange` 0 (- (`KismetArrayLibrary.Array_Length` Players) 1)))))

(fn `UserConstructionScript`)