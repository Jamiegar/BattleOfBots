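; BP_Target is a target actor that wanders horizontally and can explode, with detonation on a test key.
; A Move timeline drives swept movement toward random points, picking another on blocking hit, arrival or finish until a delay clears CanMove.
; ExplosionRadius overlaps track nearby actors in PlayersInRadius.
; Pressing G loops over them, printing damage messages without applying damage and calling DestroyActor on itself inside the loop.
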(event `self.ReceiveBeginPlay`
  ;[1 1 1] Begin Play
  (`|ExecutionSequence`
    (:`then_0`
      (`self.EnableInput` (`GameplayStatics.GetPlayerController` 0)))
    (:`then_1`
      (`self.MoveToRandomLocation`)
      (`KismetSystemLibrary.Delay` (`self.MoveDuration`))
      (set `self.CanMove` false))))

(event `MoveToRandomLocation`
  ;[1 1 1] moves target a random distance in a random direction
  (if (`self.CanMove`)
    (bind _output_get (set `self.CurrentLocation` (`self.K2_GetActorLocation`)))
    (set `self.TargetLocation` (+ _output_get (* (`KismetMathLibrary.MakeVector` (.x (`KismetMathLibrary.RandomUnitVector`)) (.y (`KismetMathLibrary.RandomUnitVector`))) (`KismetMathLibrary.RandomFloatInRange` (`self.MinDistance`) (`self.MaxDistance`)))))
    (bind (_direction _alpha) (`Timeline|Move` :!via `PlayFromStart`)
      (:`Update`
        (bind _sweephitresult (`self.K2_SetActorLocation` (`KismetMathLibrary.VInterpTo_Constant` (`self.CurrentLocation`) (`self.TargetLocation`) _alpha (`self.MoveSpeed`)) true))
        (if (or (`GameplayStatics.BreakHitResult` _sweephitresult) (== (`self.K2_GetActorLocation`) (`self.TargetLocation`)))
          (`self.MoveToRandomLocation`)))
      (:`Finished`
        (`self.MoveToRandomLocation`)))))

(event `self.ExplosionRadius.OnComponentBeginOverlap`
  (params (OverlappedComponent :type "PrimitiveComponent Object Reference") (OtherActor :type "Actor Object Reference") (OtherComp :type "PrimitiveComponent Object Reference") (OtherBodyIndex :type Integer) (bFromSweep :type Boolean) (SweepResult :type "HitResult Structure (by ref)"))
  ;[1 1 1] Store actors within radius of the blast
  (`KismetArrayLibrary.Array_AddUnique` (`self.PlayersInRadius`) OtherActor))

(event `self.ExplosionRadius.OnComponentEndOverlap`
  (params (OverlappedComponent :type "PrimitiveComponent Object Reference") (OtherActor :type "Actor Object Reference") (OtherComp :type "PrimitiveComponent Object Reference") (OtherBodyIndex :type Integer))
  ;[1 1 1] Store actors within radius of the blast
  (`KismetArrayLibrary.Array_RemoveItem` (`self.PlayersInRadius`) OtherActor))

(event `Key|G`
  (params (Key :type "Key Structure"))
  ;[1 1 1] testing purposes
  (:`Pressed`
    ;[1 1 1] detonate and damage actors within explosion radius
    (for _array_element (`self.PlayersInRadius`)
      (`KismetSystemLibrary.PrintString` (`KismetTextLibrary.Conv_TextToString` (`|FormatText` "{Actor} was damaged in explosion" _array_element)))
      (`self.K2_DestroyActor`))))

(fn `UserConstructionScript`)