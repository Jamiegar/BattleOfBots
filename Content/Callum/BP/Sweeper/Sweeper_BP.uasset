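; Sweeper hazard actor that moves into position, spins, and ragdolls characters that overlap it.
; On BeginPlay one timeline slides the Sweeper component along local X, then starts a second that rotates it about Z on each update.
; The rotation update also feeds a 15-second Delay, which starts a third timeline sliding it back along X.
; Overlap gets the character through GetCharacterMessage and calls its RagdollPlayerED.
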(event `self.ReceiveBeginPlay`
  (`Timeline|Move into postion`
    (:`Update`
      (`SceneComponent.K2_AddRelativeLocation` (`self.Sweeper`) (6.0 0.0 0.0) false false))
    (:`Finished`
      (`Timeline|Rotate`
        (:`Update`
          (`SceneComponent.K2_AddLocalRotation` (`self.Sweeper`) (struct :`Yaw` 1.0) false false)
          (`KismetSystemLibrary.Delay` 15.0)
          (`Timeline|Timeline_0`
            (:`Update`
              (`SceneComponent.K2_AddRelativeLocation` (`self.Sweeper`) (-11.0 0.0 0.0) false false))))))))

(event `self.ReceiveActorBeginOverlap`
  (params (OtherActor :type "Actor Object Reference"))
  (bind _character (message `/Game/Jamie/Interfaces/Character/BPI_Character.GetCharacter` OtherActor))
  (`/Engine/EditorBlueprintResources/StandardMacros.IsValid` _character
    (:`Is Valid`
      (`/Game/Callum/Characters/BP_BotCharacter.Ragdoll Player ED` _character))))

(fn `GetCharacter`
  (returns (Character :type "/Game/Callum/Characters/BP_BotCharacter Object Reference"))
  (return null))

(fn `GetLives`
  (returns (Lives :type "Float (double-precision)"))
  (return 0.0))

(fn `UserConstructionScript`)