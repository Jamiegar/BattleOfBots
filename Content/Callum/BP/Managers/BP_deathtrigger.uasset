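; BP_deathtrigger is an overlap volume that handles characters and other actors falling.
; Actors implementing BPI_Ragdoll go through CharcterFall, which disables ragdoll, calls OnCharacterFall, shakes BP_PlayerViewportCamera actors, sends an invisibility message to the event manager and plays a death sound.
; Otherwise, actors implementing BPI_MapFall receive a reset message.
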(event `self.Trigger.OnComponentBeginOverlap`
  (params (OverlappedComponent :type "PrimitiveComponent Object Reference") (OtherActor :type "Actor Object Reference") (OtherComp :type "PrimitiveComponent Object Reference") (OtherBodyIndex :type Integer) (bFromSweep :type Boolean) (SweepResult :type "HitResult Structure (by ref)"))
  ;[1 1 1] Each time a character falls this is called
  (if (`KismetSystemLibrary.DoesImplementInterface` OtherActor "/Game/Callum/BPI/BPI_Ragdoll.BPI_Ragdoll_C")
    (`self.CharcterFall` OtherActor)
    (elif (`KismetSystemLibrary.DoesImplementInterface` OtherActor "/Game/Jamie/Interfaces/Map/BPI_MapFall.BPI_MapFall_C")
      (message `/Game/Jamie/Interfaces/Map/BPI_MapFall.ResetActor` OtherActor))))

(event `CharcterFall`
  (params (HitActor :type "Actor Object Reference"))
  (if (`KismetSystemLibrary.DoesImplementInterface` HitActor "/Game/Callum/BPI/BPI_Ragdoll.BPI_Ragdoll_C")
    (message `/Game/Callum/BPI/BPI_Ragdoll.Disable Ragdoll` HitActor)
    (`self.OnCharacterFall` HitActor)
    (bind _outactors (`GameplayStatics.GetAllActorsOfClass` "/Game/Jamie/Blueprint/Camera/BP_PlayerViewportCamera.BP_PlayerViewportCamera_C"))
    (`/Game/Jamie/Blueprint/Camera/BP_PlayerViewportCamera.Camera Shake Quick ED` _outactors)
    (message `/Game/Callum/BPI/Invisibility_BPI.Invisibility Func` (`self.Event Manager Ref`))
    (`GameplayStatics.PlaySound2D` "/Game/Callum/Music/Sounds/Falling_Death.Falling_Death" 1.0 1.0 0.0 null null)
    (else
      (message `/Game/Jamie/Interfaces/Map/BPI_MapFall.ResetActor` HitActor))))

(fn `UserConstructionScript`)