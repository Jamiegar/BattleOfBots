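; Lives manager actor that handles character falls, respawns and last-player-standing win detection.
; On Init it converts respawn and spectator points from actor-relative to world space and binds to each death trigger's fall event.
; A fall decrements the character's lives via messages, then teleports it to the respawn point or, when out of lives, the spectator point.
; Eliminated characters leave an alive list lazily filled from the game mode, and the last one remaining triggers the win event.
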(event `/Game/Jamie/Interfaces/GameMode/BPI_Initalize.Init`
  ;[1 1 1] Initalized
  (if (`KismetArrayLibrary.Array_IsValidIndex` (`self.deathTrigger`))
    (`self.ConvertRespawnPointsToWorldSpace`)
    (for _array_element (`self.deathTrigger`)
      (add `/Game/Callum/BP/Managers/BP_deathtrigger.OnCharacterFall` _array_element (`|CreateDelegate` :!event `OnCharacterFalls`)) ; Bind to the event called in the fall trigger\nbox that is called each time a character falls
    )))

(event `OnCharacterFalls`
  (params (Character :type "Actor Object Reference"))
  ;[1 1 1] This runs each time a character falls
  (bind _output_get (set `self.character` Character))
  ;;[1 1 1] gets the lives for the falling character
  (bind _lives (message `/Game/Jamie/Interfaces/Character/BPI_Character.GetLives` _output_get))
  (`self.Check Lives` _lives))

(event `Check Lives`
  (params (Lives :type "Float (double-precision)"))
  ;[1 1 1] Reduce the number of lives and telport the character to the correct place
  (bind _result (`/Engine/EditorBlueprintResources/StandardMacros.DecrementFloat` Lives)
    (:`  `
      (message `/Game/Jamie/Interfaces/Character/BPI_Character.SetLives` (`self.character`) _result)
      (if (<= _result 0.0)
        ;;[1 1 1] Teleport to spectator point
        (`self.K2_TeleportTo` :`self` (`self.character`) :`DestLocation` (`self.spectatorPoint`))
        (`self.CheckNumberOfPlayersLeft` (`self.character`))
        (else
          ;;[1 1 1] Teleport to respawn point
          (`self.K2_TeleportTo` :`self` (`self.character`) :`DestLocation` (`self.respawnPoint`)))))))

(fn `CheckNumberOfPlayersLeft`
  (params (DeadCharacter :type "Actor Object Reference"))
  (if (not (`KismetArrayLibrary.Array_IsValidIndex` (`self.AliveCharcters`)))
    (bind _currentgamemode (message `/Game/Jamie/Interfaces/GameMode/BPI_BotsGameMode.GetGameMode` (`GameplayStatics.GetGameMode`)))
    (set `self.AliveCharcters` (`/Game/Jamie/Blueprint/GameMode/GM_Base_BrawlOfBots.character` _currentgamemode)))
  (`KismetArrayLibrary.Array_RemoveItem` (`self.AliveCharcters`) (`local.DeadCharacter`))
  (if (<= (`KismetArrayLibrary.Array_Length` (`self.AliveCharcters`)) 1)
    (`KismetSystemLibrary.PrintString` "We have a winner" true true (struct :`G` 1.0 :`B` 0.068575 :`A` 1.0) 5.0)
    (`self.OnCharacterHasWon` (`|GetArrayItem` (`self.AliveCharcters`)))))

(fn `ConvertRespawnPointsToWorldSpace`
  (set `self.respawnPoint` (+ (`self.respawnPoint`) (`self.K2_GetActorLocation`)))
  (set `self.spectatorPoint` (+ (`self.spectatorPoint`) (`self.K2_GetActorLocation`))))

(fn `UserConstructionScript`)