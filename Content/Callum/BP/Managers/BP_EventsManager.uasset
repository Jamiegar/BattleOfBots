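; BP_EventsManager is a manager that spawns timed map hazards, alternating between a sweeper and a ball rush.
; Init plays music and starts two looping timers, one triggering events and one stepping the interval enum down toward five seconds.
; The ball rush also messages the large door and raising platform.
; Interval changes update Time but never reset the running timers, and RunEvent is an empty, unused stub.
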(event `ChangeEventTimes`
  ;[0.5745 1 0.473] Enum Counting
  (bind _output_get (set `self.Time Between Events` (cast `/Game/Callum/BP/Managers/TimeBetweenEvents_Enum` (- (`self.Time Between Events`) 1))))
  (`|ExecutionSequence`
    (:`then_0`
      ;[0.7443 0.4686 1] Time Between Events Enum
      (bind _output_get_2 (set `self.Time` (select `/Game/Callum/BP/Managers/TimeBetweenEvents_Enum` (`self.Time Between Events`) :`NewEnumerator0` 5.0 :`NewEnumerator1` 10.0 :`NewEnumerator2` 15.0 :`NewEnumerator3` 20.0 :`NewEnumerator4` 25.0 :!type "Float (single-precision)")))
      (`KismetSystemLibrary.PrintString` (`KismetStringLibrary.Conv_DoubleToString` _output_get_2) true true (struct :`G` 0.66 :`B` 1.0 :`A` 1.0) _output_get_2))
    (:`then_1`
      (`KismetSystemLibrary.PrintString` (`|GetEnumeratorNameAsString` _output_get))
      (if (<= (`self.Time Between Events`) 0)
        (`KismetSystemLibrary.PrintString` "I've stopped at 5 secs")))))

(event `self.ReceiveTick`
  (params (DeltaSeconds :type "Float (single-precision)")))

(event `/Game/Jamie/Interfaces/GameMode/BPI_Initalize.Init`
  ;[1 0.5436 0.3412] Set timer
  (`KismetSystemLibrary.K2_SetTimer` null "Play Events" (`self.Time`) true)
  (`GameplayStatics.PlaySound2D` "/Game/Callum/Music/Jeremy_Blake_-_Powerup_.Jeremy_Blake_-_Powerup_" 1.0 1.0 0.0 null null)
  (`KismetSystemLibrary.K2_SetTimer` null "ChangeEventTimes" (`self.Time`) true))

(event `Play Events`
  ;[0.2314 0.1848 1] Events chain
  (`/Engine/EditorBlueprintResources/StandardMacros.FlipFlop`
    (:`A`
      (`|SpawnActorFromClass` "/Game/Callum/BP/Sweeper/Sweeper_BP.Sweeper_BP_C" (`self.Sweeper Loc`) "Undefined" "OverrideRootScale" null null))
    (:`B`
      (`|SpawnActorFromClass` "/Game/Callum/BP/BallRush/BP_Balls.BP_Balls_C" (`self.Ball Rush Loc`) "Undefined" "OverrideRootScale" null null)
      (message `/Game/Callum/BPI/OpenMainDoors_BPI.Open Main Doors Func` (`self.Large Door Ref`))
      (message `/Game/Callum/BPI/RaisingPlatform_BPI.Raising Platform Func` (`self.Raising Platform Ref`)))))

(fn `RunEvent`
  (params (`Map Hazard` :type "/Game/Jamie/Blueprint/MapHazards/BP_MapHazard Object Reference")))

(fn `UserConstructionScript`)