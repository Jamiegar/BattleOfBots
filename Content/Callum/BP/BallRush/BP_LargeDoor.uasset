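; BP_LargeDoor is a double gate door for BallRush that swings open and closed.
; OpenDoors plays the OpenDoor timeline, which lerps each gate's world rotation from a shared Start to its own end rotation, with GateR using EndL and GateL using EndR.
; CloseDoors reverses the same timeline from its end, and the timeline's Finished output calls the Doorfinished dispatcher.
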(event `OpenDoors`
  (bind (_direction _newtrack_0) (`Timeline|Open Door` :!via `PlayFromStart` :!label _label)
    (:`Update`
      (`SceneComponent.K2_SetWorldRotation` (`self.Gate_R`) (`KismetMathLibrary.RLerp` (`self.Start`) (`self.End_L`) _newtrack_0) false false)
      (`SceneComponent.K2_SetWorldRotation` (`self.Gate_L`) (`KismetMathLibrary.RLerp` (`self.Start`) (`self.End_R`) _newtrack_0) false false))
    (:`Finished`
      (`self.Doorfinished`))))

(event `CloseDoors`
  (goto _label :!via `ReverseFromEnd`))

(fn `UserConstructionScript`)