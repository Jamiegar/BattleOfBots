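; Raising platform actor for BallRush that moves from its current position when RaisingPlatformFunc is triggered.
; The event stores the root component's world location, then plays the MoveUp timeline.
; Each timeline update lerps the root between that start and the start plus EndLocation, so EndLocation acts as a relative offset.
; Movement is unswept, and nothing in this Blueprint calls the event.
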(event `self.ReceiveBeginPlay`)

(event `/Game/Callum/BPI/RaisingPlatform_BPI.Raising Platform Func`
  (set `self.Starting Location` (`SceneComponent.K2_GetComponentLocation` (`self.DefaultSceneRoot`)))
  (bind (_direction _newtrack_0) (`Timeline|Move up`)
    (:`Update`
      (`SceneComponent.K2_SetWorldLocation` (`self.DefaultSceneRoot`) (`KismetMathLibrary.VLerp` (`self.Starting Location`) (+ (`self.Starting Location`) (`self.End Location`)) _newtrack_0) false false))))

(fn `UserConstructionScript`)