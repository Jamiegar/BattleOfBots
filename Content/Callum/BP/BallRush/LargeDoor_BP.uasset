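; LargeDoor_BP is a double gate for BallRush that swings open when OpenMainDoorsFunc fires, then swings back after a delay.
; Chained timelines drive GateL and GateR in opposite yaw directions, each started from the previous one's Update pin, with the Delay before the reverse pair.
; Timelines serve only as per-frame pulses adding fixed rotation steps, so the swing depends on timeline length and frame rate.
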(event `/Game/Callum/BPI/OpenMainDoors_BPI.Open Main Doors Func`
  (bind _returnvalue (`GameplayStatics.GetWorldDeltaSeconds`))
  (`Timeline|Open Door` :`NewTime` _returnvalue
    (:`Update`
      (`SceneComponent.K2_AddWorldRotation` (`self.Gate_L`) (struct :`Yaw` 0.5) false false)
      (`Timeline|Timeline_0` :`NewTime` _returnvalue
        (:`Update`
          (`SceneComponent.K2_AddWorldRotation` (`self.Gate_R`) (struct :`Yaw` -0.5) false false)
          (`KismetSystemLibrary.Delay` 10.0)
          (`Timeline|Timeline_1`
            (:`Update`
              (`SceneComponent.K2_AddWorldRotation` (`self.Gate_L`) (struct :`Yaw` -0.5) false false)
              (`Timeline|Timeline_2`
                (:`Update`
                  (`SceneComponent.K2_AddWorldRotation` (`self.Gate_R`) (struct :`Yaw` 0.5) false false))))))))))

(fn `UserConstructionScript`)