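; BP_MapManager is a map manager Blueprint that starts grid generation on BeginPlay through GenrateCircularGrid.
; That function calls the LoopSquareGrid macro, a nested loop over GridDimentions that outputs X/Y indices; no circular filtering or loop body is wired.
; SpawnNode spawns a Node actor at a world position and stores it in TilesGrid by grid position, but nothing here calls it yet.
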(event `self.ReceiveBeginPlay`
  (`self.GenrateCircularGrid`))

(fn `GenrateCircularGrid`
  (`self.LoopSquareGrid`))

(fn `SpawnNode`
  (params (GridPos :type "/Game/Structs/Struct_GridPosition Structure") (WorldPosition :type "Vector Structure"))
  (bind _returnvalue (`|SpawnActorFromClass` (`self.node`) (`KismetMathLibrary.MakeTransform` WorldPosition) "Undefined" "OverrideRootScale" null null))
  (`BlueprintMapLibrary.Map_Add` (`self.tilesGrid`) GridPos _returnvalue))

(fn `UserConstructionScript`)